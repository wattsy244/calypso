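; Base editor build actor for the LevelDesigner tools: builds a Geometry Script dynamic mesh and bakes it to static mesh assets.
; Construction shows either the editable dynamic mesh or the baked mesh; rebuild resets to a cube, with material hooks left empty.
; Generate functions create uniquely named assets with Nanite, collision and materials, one also spawning an actor, while BakeToStaticMesh overwrites the current target.
; A standalone helper removes degenerate triangles using squared cross-product length.
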(event `ClearMaterials`)

(event `self.OnRebuildGeneratedMesh`
  (params (TargetMesh :type "DynamicMesh Object Reference"))
  (if (`self.Active?`)
    (bind _returnvalue (`BaseDynamicMeshComponent.GetDynamicMesh` (`self.DynamicMeshComponent`)))
    (`DynamicMesh.ResetToCube` _returnvalue)))

(event `ED Generate Static Mesh Event`
  (`self.GenerateNewStaticMesh` "Mesh"))

(fn `ApplyMaterials`
  (params (Materials :type "Array of MaterialInterface Object Reference")))

(fn `BakeToStaticMesh`
  (bind _returnvalue (`BaseDynamicMeshComponent.GetDynamicMesh` (`self.DynamicMeshComponent`)))
  (`GeometryScriptLibrary_StaticMeshFunctions.CopyMeshToStaticMesh` _returnvalue (`self.TargetStaticMesh`) (make `GeometryScriptCopyMeshToAssetOptions` false false false false _ _ true (make `GeometryScriptNaniteOptions` (`self.Enable Nanite`) (`self.NaniteFallBackPercent`))) (struct) null
    (:`Success`
      (for (_array_element _array_index) (`MeshComponent.GetMaterials` (`self.DynamicMeshComponent`))
        (`StaticMesh.SetMaterial` (`self.TargetStaticMesh`) _array_index _array_element))
      (`GeometryScriptLibrary_CollisionFunctions.SetStaticMeshCollisionFromComponent` (`self.TargetStaticMesh`) (`self.DynamicMeshComponent`) (make `GeometryScriptSetSimpleCollisionOptions` true) null))))

(fn `CleanDegenerateTris`
  (params (Mesh :type "DynamicMesh Object Reference") (SafeNormalTolerance :type "Float (double-precision)" :default 0.0005) (DebugLogCount :type Boolean) (DeleteDegenerates :type Boolean :default true))
  (locals (DegenerateTriList :type "Array of Integer"))
  (bind _triangleidlist (`GeometryScriptLibrary_MeshQueryFunctions.GetAllTriangleIDs` Mesh))
  (bind _indexarray (`GeometryScriptLibrary_ListUtilityFunctions.ConvertIndexListToArray` _triangleidlist))
  (for _array_element _indexarray
    (bind (_bisvalidtriangle _vertex1 _vertex2 _vertex3) (`GeometryScriptLibrary_MeshQueryFunctions.GetTrianglePositions` (`local.Mesh`) _array_element))
    (`/Engine/EditorBlueprintResources/StandardMacros.CompareFloat` (`KismetMathLibrary.VSizeSquared` (`KismetMathLibrary.Cross_VectorVector` (- _vertex3 _vertex1) (- _vertex2 _vertex1))) (`local.SafeNormalTolerance`)
      (:`<`
        (`KismetArrayLibrary.Array_Add` (`local.DegenerateTriList`) _array_element))))
  (if (not (`KismetArrayLibrary.Array_IsEmpty` (`local.DegenerateTriList`)))
    (`|ExecutionSequence`
      (:`then_0`
        (if (`local.DebugLogCount`)
          (`KismetSystemLibrary.PrintString` (`KismetStringLibrary.Concat_StrStr` (`KismetStringLibrary.Concat_StrStr` "Found " (`KismetStringLibrary.Conv_IntToString` (`KismetArrayLibrary.Array_Length` (`local.DegenerateTriList`)))) " Degenerates"))))
      (:`then_1`
        (if (`local.DeleteDegenerates`)
          (bind _indexlist (`GeometryScriptLibrary_ListUtilityFunctions.ConvertArrayToIndexList` (`local.DegenerateTriList`) "Triangle"))
          (bind (_numdeleted _returnvalue) (`GeometryScriptLibrary_MeshBasicEditFunctions.DeleteTrianglesFromMesh` (`local.Mesh`) _indexlist))
          (`GeometryScriptLibrary_MeshRepairFunctions.CompactMesh` _returnvalue null))))))

(fn `Generate`
  (bind _returnvalue (`KismetTextLibrary.Conv_TextToString` (`|FormatText` "{PathSource}/{FullPath}" (`KismetMathLibrary.SelectString` (`KismetStringLibrary.Concat_StrStr` "/" (`self.PluginName`)) "/Game" (`self.bIsInPlugin`)) (`self.PathName`))))
  (set `self.SourceGeneratorKey` (`KismetGuidLibrary.Conv_GuidToString` (`KismetGuidLibrary.NewGuid`)))
  (bind _returnvalue_2 (`BaseDynamicMeshComponent.GetDynamicMesh` (`self.DynamicMeshComponent`)))
  (`KismetSystemLibrary.PrintString` (`KismetMathLibrary.SelectString` (`KismetStringLibrary.Concat_StrStr` _returnvalue "/Generated") _returnvalue (`self.bGeneratedSubFolder`))) ; Print for debug
  (bind _uniqueassetpathandname (`GeometryScriptLibrary_CreateNewAssetFunctions.CreateUniqueNewAssetPathName` (`KismetTextLibrary.Conv_TextToString` (`|FormatText` "{PathSource}/{FullPath}" (`KismetSystemLibrary.MakeLiteralString` (`self.File Path`)) (`KismetSystemLibrary.MakeLiteralString` (`self.Folder Name Meshes`)))) (`KismetStringLibrary.Concat_StrStr` "SM_" "Mesh") (struct) null)
    (:`Failure`
      (`KismetSystemLibrary.PrintString` "Failed to Create Asset Path"))
    (:`Success`
      (bind _returnvalue_3 (`GeometryScriptLibrary_CreateNewAssetFunctions.CreateNewStaticMeshAssetFromMesh` _returnvalue_2 _uniqueassetpathandname (make `GeometryScriptCreateNewStaticMeshAssetOptions` false false (`self.Enable Nanite`) (`self.NaniteFallBackPercent`) true (`self.Collision Mode`)) null)
        (:`Failure`
          (`KismetSystemLibrary.PrintString` "Failed to Create New Asset"))
        (:`Success`
          (bind _output_get (set `self.TargetStaticMesh` _returnvalue_3))
          (`GeometryScriptLibrary_CollisionFunctions.SetStaticMeshCollisionFromComponent` _output_get (`self.DynamicMeshComponent`) (struct :`bEmitTransaction` true) null)
          (bind _returnvalue_4 (`BaseDynamicMeshComponent.GetDynamicMesh` (`self.DynamicMeshComponent`)))
          (`GeometryScriptLibrary_StaticMeshFunctions.CopyMeshToStaticMesh` _returnvalue_4 (`self.TargetStaticMesh`) (make `GeometryScriptCopyMeshToAssetOptions` false false false true (`MeshComponent.GetMaterials` (`self.DynamicMeshComponent`))) (struct) null
            (:`Success`
              ;[1 1 1] Add materials
              (for (_array_element _array_index) (`MeshComponent.GetMaterials` (`self.DynamicMeshComponent`))
                (`StaticMesh.SetMaterial` (`self.TargetStaticMesh`) _array_index _array_element))
              (return))))))))

(fn `GenerateNewStaticMesh`
  (params (BaseAssetName :type String :default "Mesh") (Transform :type "Transform Structure"))
  (returns (`Static Mesh Actor` :type "StaticMeshActor Object Reference"))
  (set `self.SourceGeneratorKey` (`KismetGuidLibrary.Conv_GuidToString` (`KismetGuidLibrary.NewGuid`)))
  (bind _returnvalue (`BaseDynamicMeshComponent.GetDynamicMesh` (`self.DynamicMeshComponent`)))
  (bind _uniqueassetpathandname (`GeometryScriptLibrary_CreateNewAssetFunctions.CreateUniqueNewAssetPathName` (`KismetTextLibrary.Conv_TextToString` (`|FormatText` "{PathSource}/{FullPath}" (`KismetSystemLibrary.MakeLiteralString` (`self.File Path`)) (`KismetSystemLibrary.MakeLiteralString` (`self.Folder Name Meshes`)))) (`KismetStringLibrary.Concat_StrStr` "SM_" (`local.BaseAssetName`)) (struct) null)
    (:`Failure`
      (`KismetSystemLibrary.PrintString` "Failed to Create Asset Path"))
    (:`Success`
      (bind _returnvalue_2 (`GeometryScriptLibrary_CreateNewAssetFunctions.CreateNewStaticMeshAssetFromMesh` _returnvalue _uniqueassetpathandname (make `GeometryScriptCreateNewStaticMeshAssetOptions` false false (`self.Enable Nanite`) (`self.NaniteFallBackPercent`) true (`self.Collision Mode`)) null)
        (:`Failure`
          (`KismetSystemLibrary.PrintString` "Failed to Create New Asset"))
        (:`Success`
          (bind _output_get (set `self.TargetStaticMesh` _returnvalue_2))
          (`GeometryScriptLibrary_CollisionFunctions.SetStaticMeshCollisionFromComponent` _output_get (`self.DynamicMeshComponent`) (struct :`bEmitTransaction` true) null)
          (bind _returnvalue_3 (`BaseDynamicMeshComponent.GetDynamicMesh` (`self.DynamicMeshComponent`)))
          (`GeometryScriptLibrary_MeshTransformFunctions.TransformMesh` _returnvalue_3 (`local.Transform`) null)
          (bind _returnvalue_4 (`GeometryScriptLibrary_StaticMeshFunctions.CopyMeshToStaticMesh` _returnvalue_3 (`self.TargetStaticMesh`) (make `GeometryScriptCopyMeshToAssetOptions` true true true true (`MeshComponent.GetMaterials` (`self.DynamicMeshComponent`))) (struct) null)
            (:`Success`
              (bind _returnvalue_5 (`EditorLevelLibrary.SpawnActorFromObject` _returnvalue_4 (0.0 0.0 500.0) (.rotation (`local.Transform`))))
              (set `self.Object` _returnvalue_5)
              (bind _asstatic_mesh_actor (cast `StaticMeshActor` (`self.Object`)))
              ;[1 1 1] Add materials
              (for (_array_element _array_index) (`MeshComponent.GetMaterials` (`self.DynamicMeshComponent`))
                (`StaticMesh.SetMaterial` (`self.TargetStaticMesh`) _array_index _array_element))
              (return _asstatic_mesh_actor))))))))

(fn `UserConstructionScript`
  (`SceneComponent.SetVisibility` (`self.DynamicMeshComponent`) (`self.Editable`) false)
  (`SceneComponent.SetVisibility` (`self.BakedMesh`) (not (`self.Editable`)) false)
  (`StaticMeshComponent.SetStaticMesh` (`self.BakedMesh`) (`self.TargetStaticMesh`)))