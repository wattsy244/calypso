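; Generated dynamic-mesh level design tool that repeats boxes at even intervals along a spline, with optional polygroup bevel.
; On rebuild, box locations feed MakeCollisionSpansPointSet, which merges near-straight runs into spans using a direction dot-product tolerance.
; A profile is swept along each span to build simplified swept-hull collision, or appended as a debug-material preview meant to be off before baking.
; Disabling simplified collision resets the component's collision.
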(event `self.ClearMaterials`
  (bind _height (`self.Height`))
  (bind _numberofpieces (`self.NumberOfPieces`))
  (bind _returnvalue (+ _height (`self.CollisionDepthAdditive`)))
  (bind _returnvalue_2 (+ (`self.Width`) (`self.CollisionWidthAdditive`)))
  (bind _returnvalue_3 (* (+ _height (`self.OffsetCollision`)) -1.0))
  ;[1 1 1] Clear Materials
  (set `self.Material` null)
  (bind _returnvalue_4 (`DynamicMesh.Reset` (stale `self.OnRebuildGeneratedMesh` TargetMesh) :!label _label))
  (set `self.Target Mesh` _returnvalue_4)
  (bind _returnvalue_5 (`self.AllocateComputeMesh`))
  (set `self.CollisionSweep` _returnvalue_5)
  ;[1 1 1] Append Mesh Over spline
  (set `self.i` (/ 1.0 (`KismetMathLibrary.Conv_IntToDouble` _numberofpieces)))
  (for _index (range 1 _numberofpieces)
    (bind (_returnvalue_location _returnvalue_rotation) (`KismetMathLibrary.BreakTransform` (`SplineComponent.GetTransformAtTime` (`self.Spline`) (`KismetMathLibrary.FClamp` (* _index (`self.i`))) "Local" true false)))
    (bind _returnvalue_6 (`GeometryScriptLibrary_MeshPrimitiveFunctions.AppendBox` (`self.Target Mesh`) (struct) (`KismetMathLibrary.MakeTransform` (+ _returnvalue_location (`self.Start Offset`)) _returnvalue_rotation) (`self.Depth`) (`self.Width`) (`self.Height`) 0 0 0 "Base" null))
    (set `self.Target Mesh` _returnvalue_6)
    ;[1 1 1] Prep Spline For Collision
    (`KismetArrayLibrary.Array_Add` (`self.Direction`) _returnvalue_location))
  ;[1 1 1] Bevel
  (if (`self.bBevel`)
    (bind _returnvalue_7 (`GeometryScriptLibrary_MeshModelingFunctions.ApplyMeshPolygroupBevel` (`self.Target Mesh`) (make `GeometryScriptMeshBevelOptions` (`self.Options Bevel Distance`)) null))
    (set `self.Target Mesh` _returnvalue_7))
  ;[1 1 1] Collision Sweep
  (set `self.CollisionShape` (`|MakeArray` (`KismetMathLibrary.MakeVector2D` 0.0 _returnvalue_3) (`KismetMathLibrary.MakeVector2D` _returnvalue_2 _returnvalue_3) (`KismetMathLibrary.MakeVector2D` _returnvalue_2 _returnvalue) (`KismetMathLibrary.MakeVector2D` 0.0 _returnvalue) :!type "Vector2D Structure"))
  (set `self.CollisionOffset` (/ _returnvalue_2 -2.0))
  (bind (_startpoints _endpoints) (`self.MakeCollisionSpansPointSet` (`self.Direction`) (`self.CollisionGeoTolerance`)))
  (set `self.CollisionStartPoints` _startpoints)
  (bind _output_get (set `self.CollisionEndPoints` _endpoints))
  (for _index_2 (range (`KismetArrayLibrary.Array_Length` _output_get))
    (`GeometryScriptLibrary_MeshPrimitiveFunctions.AppendSimpleSweptPolygon` (`self.CollisionSweep`) (make `GeometryScriptPrimitiveOptions` "SingleGroup") (`KismetMathLibrary.MakeTransform` (`KismetMathLibrary.MakeVector` (`self.CollisionOffset`))) (`self.CollisionShape`) (`|MakeArray` (`|GetArrayItem` (`self.CollisionStartPoints`) _index_2) (`|GetArrayItem` (`self.CollisionEndPoints`) _index_2)) false true 1.0 1.0 null))
  (bind _returnvalue_8 (`GeometryScriptLibrary_MeshMaterialFunctions.RemapMaterialIDs` (`self.CollisionSweep`) 0 1 null))
  (set `self.CollisionSweep` _returnvalue_8)
  (if (`self.SimplifiedCollision`)
    ;[1 1 1] Collision And Collision preview
    (if (`self.bPreviewSimplified(turnOFFBEFOREBAKE)`)
      (bind _returnvalue_9 (`GeometryScriptLibrary_MeshMaterialFunctions.RemapMaterialIDs` (`self.CollisionSweep`) 0 1 null))
      (bind _returnvalue_10 (`GeometryScriptLibrary_MeshBasicEditFunctions.AppendMesh` (`self.Target Mesh`) _returnvalue_9 (struct) false null))
      (set `self.Target Mesh` _returnvalue_10)
      (else
        (bind _returnvalue_11 (`GeometryScriptLibrary_CollisionFunctions.SetDynamicMeshCollisionFromMesh` (`self.CollisionSweep`) (`self.DynamicMeshComponent`) (make `GeometryScriptCollisionFromMeshOptions` false "SweptHulls" false false false 1.0 false 25 0.5 "X" false 50) null))
        (set `self.Target Mesh` _returnvalue_11)))
    (else
      (`GeometryScriptLibrary_CollisionFunctions.ResetDynamicMeshCollision` (`self.DynamicMeshComponent`) false null)))
  (`self.ReleaseAllComputeMeshes`)
  ;[1 1 1] Apply Materials
  (`DynamicMeshComponent.ConfigureMaterialSet` (`self.DynamicMeshComponent`) (`|MakeArray` (`self.Material`) "/Game/LevelDesigner/Demo/Materials/M_DebugTool.M_DebugTool"))
  (`self.CleanDegenerateTris` (`self.Target Mesh`)))

(event `self.OnRebuildGeneratedMesh`
  (params (TargetMesh :type "DynamicMesh Object Reference"))
  (goto _label))

(fn `ApplyMaterials`
  (params (Materials :type "Array of MaterialInterface Object Reference (by ref)"))
  (set `self.Material` (`|GetArrayItem` Materials))
  (return))

(fn `MakeCollisionSpansPointSet`
  (params (InputPoints :type "Array of Vector Structure") (LineDeviationTol :type "Float (double-precision)" :default 0.95))
  (returns (StartPoints :type "Array of Vector Structure") (EndPoints :type "Array of Vector Structure"))
  (locals (ArrayLastIndex :type Integer :default 0) (SpanStartPoint :type "Vector Structure") (FirstInSpan :type Boolean) (OutStartPoints :type "Array of Vector Structure") (CurPoint :type "Vector Structure") (CurDirection :type "Vector Structure") (LineDirection :type "Vector Structure") (PrevPoint :type "Vector Structure") (OutEndPoints :type "Array of Vector Structure"))
  (set `local.ArrayLastIndex` (- (`KismetArrayLibrary.Array_Length` InputPoints) 1))
  (bind _output_get (set `local.SpanStartPoint` (`|GetArrayItem` (`local.InputPoints`))))
  (set `local.PrevPoint` _output_get)
  (set `local.FirstInSpan` true)
  (`KismetArrayLibrary.Array_Add` (`local.OutStartPoints`) (`local.SpanStartPoint`))
  (for _index (range 1 (+ (`local.ArrayLastIndex`) 1))
    (set `local.CurPoint` (`|GetArrayItem` (`local.InputPoints`) _index))
    (set `local.CurDirection` (`KismetMathLibrary.Normal` (- (`local.CurPoint`) (`local.PrevPoint`))))
    (if (`local.FirstInSpan`)
      (set `local.LineDirection` (`local.CurDirection`))
      (set `local.PrevPoint` (`local.CurPoint`))
      (set `local.FirstInSpan` false)
      (else
        (`/Engine/EditorBlueprintResources/StandardMacros.CompareFloat` (`KismetMathLibrary.Dot_VectorVector` (`local.CurDirection`) (`local.LineDirection`)) (`local.LineDeviationTol`)
          (:`>`
            (set `local.PrevPoint` (`local.CurPoint`) :!label _label))
          (:`==`
            (goto _label))
          (:`<`
            (`KismetArrayLibrary.Array_Add` (`local.OutEndPoints`) (`local.PrevPoint`))
            (`KismetArrayLibrary.Array_Add` (`local.OutStartPoints`) (`local.CurPoint`))
            (bind _output_get_2 (set `local.SpanStartPoint` (`local.CurPoint`)))
            (set `local.PrevPoint` _output_get_2)
            (set `local.FirstInSpan` true))))))
  (`KismetArrayLibrary.Array_Add` (`local.OutEndPoints`) (`local.PrevPoint`))
  (return (`local.OutStartPoints`) (`local.OutEndPoints`)))

(fn `UserConstructionScript`
  (`parent.UserConstructionScript`))