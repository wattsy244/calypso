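; BP_Floor is a level-design Geometry Script tool that generates a parametric floor panel sized by a Handle vector.
; On rebuild it extrudes a rounded or squared base, then booleans in an inset topper carrying a second material ID for trim/center materials.
; Options add a differently shaped half, polygroup bevels, plane cut and mirror before degenerate-triangle cleanup.
; Construction writes Handle dimensions to a BP_Dimensions child actor's text.
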(event Custom|Update%20UI%20Event
  (Utilities|FlowControl|Delay 0.05)
  (CallFunction|UpdateUI))

(event Custom|Compile
  (Utilities|FlowControl|Delay 0.05)
  (Class|BlueprintEditorLibrary|CompileBlueprint "BP_Floor"))

(event EventClearMaterials
  (bind (_location _axis) (|GetLocationAndAxis_2))
  (bind (_offsetcentery _x _y _z) (|GetInfoCutter))
  (bind (_offsetcenterx _offsetcentery_2 _x_2 _y_2 _extrude) (|GetInfoNewCorner))
  (bind (_offsetx _offsety _offsetz _x_3 _y_3) (|GetNewPiecesInfos))
  (bind (_offsetcenterx_2 _offsetcentery_3 _x_4 _y_4 _cornerradius) (|GetInfosFromVector))
  (bind (_offetcenterx _offsetcentery_4 _offsetcenterz _x_5 _y_5 _cornerradius_2) (|GetInfosFromParent))
  (bind _cutter_transform (Variables|Default|GetCutter%20Transform))
  ;[1 1 1] CLEAR MATERIALS
  (Variables|Default|Set🎨%20Material%20Trim 0)
  (Variables|Default|Set🎨%20Material%20Center 0)
  (bind _returnvalue (DynamicMeshComponent|GetDynamicMesh (Variables|Default|GetDynamicMeshComponent)))
  (bind _returnvalue_2 (DynamicMesh|Reset _returnvalue))
  ;[1 1 1] PanelBase
  (bind _returnvalue_3 (Class|GeometryScriptLibraryMeshPrimitiveFunctions|AppendRoundRectangleCompatibility50 _returnvalue_2 (Utilities|Struct|MakeGeometryScriptPrimitiveOptions "PerFace" false "Uniform") (Math|Transform|MakeTransform (Math|Vector|MakeVector _offsetcenterx_2 _offsetcentery_3 0.0) "0, 0, 0" "1.000000,1.000000,1.000000") _x_4 _y_4 _cornerradius 0 0 (Variables|Default|Get⚙%20Steps) 0))
  (Variables|Essentials|SetDynamicMesh _returnvalue_3)
  (if (Variables|Default|Get⚙%20bRec)
    (bind _returnvalue_4 (Class|GeometryScriptLibraryMeshSimplifyFunctions|ApplySimplifytoTriangleCount (Variables|Essentials|GetDynamicMesh) 2 (Utilities|Struct|MakeGeometryScriptSimplifyMeshOptions "AttributeAware" true true true false false) 0))
    (Variables|Essentials|SetDynamicMesh _returnvalue_4))
  (bind _returnvalue_5 (Class|GeometryScriptLibraryMeshModelingFunctions|ApplyMeshExtrude (Variables|Essentials|GetDynamicMesh) (Utilities|Struct|MakeGeometryScriptMeshExtrudeOptions (.z (Variables|Default|Get⚙%20Handle)) "0.000000,0.000000,1.000000" 1.0 true) 0))
  (Variables|Essentials|SetDynamicMesh _returnvalue_5)
  (if (Variables|Default|Get📐%20Bevel%20Panel)
    (bind _target_mesh (CallFunction|FnBevel (Variables|Essentials|GetDynamicMesh) (Variables|Default|Get📐%20Bevel%20Distance%20Panel)))
    (Variables|Essentials|SetDynamicMesh _target_mesh))
  ;[1 1 1] Topper
  (bind _returnvalue_6 (DynamicMeshActor|AllocateComputeMesh))
  (bind _returnvalue_7 (Class|GeometryScriptLibraryMeshPrimitiveFunctions|AppendRoundRectangleCompatibility50 :TargetMesh _returnvalue_6 :Transform (Math|Transform|MakeTransform (Math|Vector|MakeVector _offetcenterx _offsetcentery_4 _offsetcenterz) "0, 0, 0" "1.000000,1.000000,1.000000") :DimensionX _x_5 :DimensionY _y_5 :CornerRadius _cornerradius_2 :StepsRound (Variables|Default|Get⚙%20Steps) :Debug 0))
  (Variables|Essentials|SetTarget%20Mesh _returnvalue_7)
  (if (Variables|Default|Get⚙%20Square%20Top?)
    (bind _returnvalue_8 (Class|GeometryScriptLibraryMeshSimplifyFunctions|ApplySimplifytoTriangleCount (Variables|Essentials|GetTarget%20Mesh) 2 (Utilities|Struct|MakeGeometryScriptSimplifyMeshOptions "AttributeAware" true true true false false) 0))
    (Variables|Essentials|SetTarget%20Mesh _returnvalue_8))
  (bind _returnvalue_9 (Class|GeometryScriptLibraryMeshModelingFunctions|ApplyMeshExtrude (Variables|Essentials|GetTarget%20Mesh) (Utilities|Struct|MakeGeometryScriptMeshExtrudeOptions (Variables|Default|Get⚙%20TopperExtrude) "0.000000,0.000000,1.000000" 1.0 true) 0))
  (bind _returnvalue_10 (GeometryScript|Materials|EnableMaterialIDs _returnvalue_9 0))
  (bind _returnvalue_11 (GeometryScript|Materials|RemapMaterialIDs _returnvalue_10 0 1 0))
  (Variables|Essentials|SetTarget%20Mesh _returnvalue_11)
  (if (Variables|Default|Get📐%20Bevel%20Topper)
    (bind _target_mesh_2 (CallFunction|FnBevel (Variables|Essentials|GetTarget%20Mesh) (Variables|Default|Get📐%20Bevel%20Distance%20Topper)))
    (Variables|Essentials|SetTarget%20Mesh _target_mesh_2))
  (bind _returnvalue_12 (GeometryScript|Booleans|ApplyMeshBoolean :TargetMesh _returnvalue_5 :ToolMesh (Variables|Essentials|GetTarget%20Mesh) :Operation (Variables|Default|Get⚙%20Operation) :Debug 0))
  (switch Utilities|FlowControl|Switch|SwitchonE_PanelType (Variables|Default|Get⚙%20Apply%20Settings) ; Decide if we want the other half to be same or of different type
    (:NewEnumerator0
      _)
    (:NewEnumerator1
      ;[1 1 1] Different Half
      (bind _returnvalue_13 (DynamicMeshActor|AllocateComputeMesh))
      (bind _returnvalue_14 (Class|GeometryScriptLibraryMeshPrimitiveFunctions|AppendBox :TargetMesh _returnvalue_13 :Transform (Math|Transform|MakeTransform (Math|Vector|MakeVector 0.0 _offsetcentery 0.0) "0, 0, 0" "1.000000,1.000000,1.000000") :DimensionX _x :DimensionY _y :DimensionZ _z :Debug 0))
      (bind _returnvalue_15 (GeometryScript|Booleans|ApplyMeshBoolean :TargetMesh _returnvalue_12 :ToolMesh _returnvalue_14 :Operation "Subtract" :Debug 0))
      (bind _returnvalue_16 (DynamicMeshActor|AllocateComputeMesh))
      (bind _returnvalue_17 (Class|GeometryScriptLibraryMeshPrimitiveFunctions|AppendRectangleCompatibility50 :TargetMesh _returnvalue_16 :Transform (Math|Transform|MakeTransform (Math|Vector|MakeVector _offsetcenterx _offsetcentery_2 0.0) "0, 0, 0" "1.000000,1.000000,1.000000") :DimensionX _x_2 :DimensionY _y_2 :Debug 0))
      (bind _returnvalue_18 (Class|GeometryScriptLibraryMeshModelingFunctions|ApplyMeshExtrude _returnvalue_17 (Utilities|Struct|MakeGeometryScriptMeshExtrudeOptions _extrude "0.000000,0.000000,1.000000" 1.0 true) 0))
      (bind _returnvalue_19 (GeometryScript|Booleans|ApplyMeshBoolean :TargetMesh _returnvalue_15 :ToolMesh _returnvalue_18 :Operation "Union" :Debug 0))
      (bind _returnvalue_20 (DynamicMeshActor|AllocateComputeMesh))
      (bind _returnvalue_21 (Class|GeometryScriptLibraryMeshPrimitiveFunctions|AppendRectangleCompatibility50 :TargetMesh _returnvalue_20 :Transform (Math|Transform|MakeTransform (Math|Vector|MakeVector _offsetx _offsety _offsetz) "0, 0, 0" "1.000000,1.000000,1.000000") :DimensionX _x_3 :DimensionY _y_3 :Debug 0))
      (bind _returnvalue_22 (Class|GeometryScriptLibraryMeshModelingFunctions|ApplyMeshExtrude _returnvalue_21 (Utilities|Struct|MakeGeometryScriptMeshExtrudeOptions (Variables|Default|Get⚙%20TopperExtrude) "0.000000,0.000000,1.000000" 1.0 true) 0))
      (bind _returnvalue_23 (GeometryScript|Materials|EnableMaterialIDs _returnvalue_22 0))
      (bind _returnvalue_24 (GeometryScript|Materials|RemapMaterialIDs _returnvalue_23 0 1 0))
      (GeometryScript|Booleans|ApplyMeshBoolean :TargetMesh _returnvalue_19 :ToolMesh _returnvalue_24 :Operation (Variables|Default|Get⚙%20Operation) :Debug 0)))
  (bind _returnvalue_25 (Class|GeometryScriptLibraryMeshNormalsFunctions|ComputeSplitNormals _returnvalue_12 (Utilities|Struct|MakeGeometryScriptSplitNormalsOptions true 25.0 false "(bDefaultLayer=True,ExtendedLayerIndex=0)") (Utilities|Struct|MakeGeometryScriptCalculateNormalsOptions true true) 0))
  (Variables|Essentials|SetDynamicMesh _returnvalue_25)
  (if (Variables|Default|Get🔪%20Use%20Cutter?)
    ;[1 1 1] Cutter
    (Class|GeometryScriptLibraryMeshBooleanFunctions|ApplyMeshPlaneCut (Variables|Essentials|GetDynamicMesh) (Math|Transform|MakeTransform (.location _cutter_transform) (.rotation _cutter_transform) "0.100000,0.100000,0.100000") (Utilities|Struct|MakeGeometryScriptMeshPlaneCutOptions false true false 1.0) 0)
    (Rendering|Debug|DrawDebugArrow (.location _cutter_transform) "0, 0, 0" 1e+01 "(R=1.000000,G=1.000000,B=1.000000,A=0.500000)" 1.0 5.0))
  (if (Variables|Default|Get📐%20Bevel%20Combine)
    (CallFunction|FnBevel (Variables|Essentials|GetDynamicMesh) (Variables|Default|Get📐%20Bevel%20Distance%20Combine)))
  (if (Variables|Default|Get👀%20Use%20Mirror?)
    ;[1 1 1] Mirror
    (bind _returnvalue_26 (Class|GeometryScriptLibraryMeshBooleanFunctions|ApplyMeshMirror (Variables|Essentials|GetDynamicMesh) (Math|Transform|MakeTransform _location _axis "1.000000,1.000000,1.000000") (Utilities|Struct|MakeGeometryScriptMeshMirrorOptions true true true) 0))
    (Variables|Essentials|SetDynamicMesh _returnvalue_26))
  (CallFunction|CleanDegenerateTris (Variables|Essentials|GetDynamicMesh) (Variables|Default|Get⚙%20Safe%20Normal%20Tolerance) false true)
  (Class|DynamicMeshComponent|ConfigureMaterialSet (Variables|Default|GetDynamicMeshComponent) (Utilities|Array|MakeArray (Variables|Default|Get🎨%20Material%20Trim) (Variables|Default|Get🎨%20Material%20Center)))
  (DynamicMeshActor|ReleaseAllComputeMeshes)
  (Transformation|AddWorldOffset (Variables|Default|GetDynamicMeshComponent) (Variables|Default|Get⚙%20Floor%20Location%20Offset) false false))

(event Events|EventOnRebuildGeneratedMesh
  (params (TargetMesh :type Dynamic%20Mesh%20Object%20Reference))
  (bind (_location _axis) (|GetLocationAndAxis_2))
  (bind (_offsetcentery _x _y _z) (|GetInfoCutter))
  (bind (_offsetcenterx _offsetcentery_2 _x_2 _y_2 _extrude) (|GetInfoNewCorner))
  (bind (_offsetx _offsety _offsetz _x_3 _y_3) (|GetNewPiecesInfos))
  (bind (_offsetcenterx_2 _offsetcentery_3 _x_4 _y_4 _cornerradius) (|GetInfosFromVector))
  (bind (_offetcenterx _offsetcentery_4 _offsetcenterz _x_5 _y_5 _cornerradius_2) (|GetInfosFromParent))
  (bind _cutter_transform (Variables|Default|GetCutter%20Transform))
  (bind _returnvalue (DynamicMeshComponent|GetDynamicMesh (Variables|Default|GetDynamicMeshComponent)))
  (bind _returnvalue_2 (DynamicMesh|Reset _returnvalue))
  ;[1 1 1] PanelBase
  (bind _returnvalue_3 (Class|GeometryScriptLibraryMeshPrimitiveFunctions|AppendRoundRectangleCompatibility50 _returnvalue_2 (Utilities|Struct|MakeGeometryScriptPrimitiveOptions "PerFace" false "Uniform") (Math|Transform|MakeTransform (Math|Vector|MakeVector _offsetcenterx_2 _offsetcentery_3 0.0) "0, 0, 0" "1.000000,1.000000,1.000000") _x_4 _y_4 _cornerradius 0 0 (Variables|Default|Get⚙%20Steps) 0))
  (Variables|Essentials|SetDynamicMesh _returnvalue_3)
  (if (Variables|Default|Get⚙%20bRec)
    (bind _returnvalue_4 (Class|GeometryScriptLibraryMeshSimplifyFunctions|ApplySimplifytoTriangleCount (Variables|Essentials|GetDynamicMesh) 2 (Utilities|Struct|MakeGeometryScriptSimplifyMeshOptions "AttributeAware" true true true false false) 0))
    (Variables|Essentials|SetDynamicMesh _returnvalue_4))
  (bind _returnvalue_5 (Class|GeometryScriptLibraryMeshModelingFunctions|ApplyMeshExtrude (Variables|Essentials|GetDynamicMesh) (Utilities|Struct|MakeGeometryScriptMeshExtrudeOptions (.z (Variables|Default|Get⚙%20Handle)) "0.000000,0.000000,1.000000" 1.0 true) 0))
  (Variables|Essentials|SetDynamicMesh _returnvalue_5)
  (if (Variables|Default|Get📐%20Bevel%20Panel)
    (bind _target_mesh (CallFunction|FnBevel (Variables|Essentials|GetDynamicMesh) (Variables|Default|Get📐%20Bevel%20Distance%20Panel)))
    (Variables|Essentials|SetDynamicMesh _target_mesh))
  ;[1 1 1] Topper
  (bind _returnvalue_6 (DynamicMeshActor|AllocateComputeMesh))
  (bind _returnvalue_7 (Class|GeometryScriptLibraryMeshPrimitiveFunctions|AppendRoundRectangleCompatibility50 :TargetMesh _returnvalue_6 :Transform (Math|Transform|MakeTransform (Math|Vector|MakeVector _offetcenterx _offsetcentery_4 _offsetcenterz) "0, 0, 0" "1.000000,1.000000,1.000000") :DimensionX _x_5 :DimensionY _y_5 :CornerRadius _cornerradius_2 :StepsRound (Variables|Default|Get⚙%20Steps) :Debug 0))
  (Variables|Essentials|SetTarget%20Mesh _returnvalue_7)
  (if (Variables|Default|Get⚙%20Square%20Top?)
    (bind _returnvalue_8 (Class|GeometryScriptLibraryMeshSimplifyFunctions|ApplySimplifytoTriangleCount (Variables|Essentials|GetTarget%20Mesh) 2 (Utilities|Struct|MakeGeometryScriptSimplifyMeshOptions "AttributeAware" true true true false false) 0))
    (Variables|Essentials|SetTarget%20Mesh _returnvalue_8))
  (bind _returnvalue_9 (Class|GeometryScriptLibraryMeshModelingFunctions|ApplyMeshExtrude (Variables|Essentials|GetTarget%20Mesh) (Utilities|Struct|MakeGeometryScriptMeshExtrudeOptions (Variables|Default|Get⚙%20TopperExtrude) "0.000000,0.000000,1.000000" 1.0 true) 0))
  (bind _returnvalue_10 (GeometryScript|Materials|EnableMaterialIDs _returnvalue_9 0))
  (bind _returnvalue_11 (GeometryScript|Materials|RemapMaterialIDs _returnvalue_10 0 1 0))
  (Variables|Essentials|SetTarget%20Mesh _returnvalue_11)
  (if (Variables|Default|Get📐%20Bevel%20Topper)
    (bind _target_mesh_2 (CallFunction|FnBevel (Variables|Essentials|GetTarget%20Mesh) (Variables|Default|Get📐%20Bevel%20Distance%20Topper)))
    (Variables|Essentials|SetTarget%20Mesh _target_mesh_2))
  (bind _returnvalue_12 (GeometryScript|Booleans|ApplyMeshBoolean :TargetMesh _returnvalue_5 :ToolMesh (Variables|Essentials|GetTarget%20Mesh) :Operation (Variables|Default|Get⚙%20Operation) :Debug 0))
  (switch Utilities|FlowControl|Switch|SwitchonE_PanelType (Variables|Default|Get⚙%20Apply%20Settings) ; Decide if we want the other half to be same or of different type
    (:NewEnumerator0
      _)
    (:NewEnumerator1
      ;[1 1 1] Different Half
      (bind _returnvalue_13 (DynamicMeshActor|AllocateComputeMesh))
      (bind _returnvalue_14 (Class|GeometryScriptLibraryMeshPrimitiveFunctions|AppendBox :TargetMesh _returnvalue_13 :Transform (Math|Transform|MakeTransform (Math|Vector|MakeVector 0.0 _offsetcentery 0.0) "0, 0, 0" "1.000000,1.000000,1.000000") :DimensionX _x :DimensionY _y :DimensionZ _z :Debug 0))
      (bind _returnvalue_15 (GeometryScript|Booleans|ApplyMeshBoolean :TargetMesh _returnvalue_12 :ToolMesh _returnvalue_14 :Operation "Subtract" :Debug 0))
      (bind _returnvalue_16 (DynamicMeshActor|AllocateComputeMesh))
      (bind _returnvalue_17 (Class|GeometryScriptLibraryMeshPrimitiveFunctions|AppendRectangleCompatibility50 :TargetMesh _returnvalue_16 :Transform (Math|Transform|MakeTransform (Math|Vector|MakeVector _offsetcenterx _offsetcentery_2 0.0) "0, 0, 0" "1.000000,1.000000,1.000000") :DimensionX _x_2 :DimensionY _y_2 :Debug 0))
      (bind _returnvalue_18 (Class|GeometryScriptLibraryMeshModelingFunctions|ApplyMeshExtrude _returnvalue_17 (Utilities|Struct|MakeGeometryScriptMeshExtrudeOptions _extrude "0.000000,0.000000,1.000000" 1.0 true) 0))
      (bind _returnvalue_19 (GeometryScript|Booleans|ApplyMeshBoolean :TargetMesh _returnvalue_15 :ToolMesh _returnvalue_18 :Operation "Union" :Debug 0))
      (bind _returnvalue_20 (DynamicMeshActor|AllocateComputeMesh))
      (bind _returnvalue_21 (Class|GeometryScriptLibraryMeshPrimitiveFunctions|AppendRectangleCompatibility50 :TargetMesh _returnvalue_20 :Transform (Math|Transform|MakeTransform (Math|Vector|MakeVector _offsetx _offsety _offsetz) "0, 0, 0" "1.000000,1.000000,1.000000") :DimensionX _x_3 :DimensionY _y_3 :Debug 0))
      (bind _returnvalue_22 (Class|GeometryScriptLibraryMeshModelingFunctions|ApplyMeshExtrude _returnvalue_21 (Utilities|Struct|MakeGeometryScriptMeshExtrudeOptions (Variables|Default|Get⚙%20TopperExtrude) "0.000000,0.000000,1.000000" 1.0 true) 0))
      (bind _returnvalue_23 (GeometryScript|Materials|EnableMaterialIDs _returnvalue_22 0))
      (bind _returnvalue_24 (GeometryScript|Materials|RemapMaterialIDs _returnvalue_23 0 1 0))
      (GeometryScript|Booleans|ApplyMeshBoolean :TargetMesh _returnvalue_19 :ToolMesh _returnvalue_24 :Operation (Variables|Default|Get⚙%20Operation) :Debug 0)))
  (bind _returnvalue_25 (Class|GeometryScriptLibraryMeshNormalsFunctions|ComputeSplitNormals _returnvalue_12 (Utilities|Struct|MakeGeometryScriptSplitNormalsOptions true 25.0 false "(bDefaultLayer=True,ExtendedLayerIndex=0)") (Utilities|Struct|MakeGeometryScriptCalculateNormalsOptions true true) 0))
  (Variables|Essentials|SetDynamicMesh _returnvalue_25)
  (if (Variables|Default|Get🔪%20Use%20Cutter?)
    ;[1 1 1] Cutter
    (Class|GeometryScriptLibraryMeshBooleanFunctions|ApplyMeshPlaneCut (Variables|Essentials|GetDynamicMesh) (Math|Transform|MakeTransform (.location _cutter_transform) (.rotation _cutter_transform) "0.100000,0.100000,0.100000") (Utilities|Struct|MakeGeometryScriptMeshPlaneCutOptions false true false 1.0) 0)
    (Rendering|Debug|DrawDebugArrow (.location _cutter_transform) "0, 0, 0" 1e+01 "(R=1.000000,G=1.000000,B=1.000000,A=0.500000)" 1.0 5.0))
  (if (Variables|Default|Get📐%20Bevel%20Combine)
    (CallFunction|FnBevel (Variables|Essentials|GetDynamicMesh) (Variables|Default|Get📐%20Bevel%20Distance%20Combine)))
  (if (Variables|Default|Get👀%20Use%20Mirror?)
    ;[1 1 1] Mirror
    (bind _returnvalue_26 (Class|GeometryScriptLibraryMeshBooleanFunctions|ApplyMeshMirror (Variables|Essentials|GetDynamicMesh) (Math|Transform|MakeTransform _location _axis "1.000000,1.000000,1.000000") (Utilities|Struct|MakeGeometryScriptMeshMirrorOptions true true true) 0))
    (Variables|Essentials|SetDynamicMesh _returnvalue_26))
  (CallFunction|CleanDegenerateTris (Variables|Essentials|GetDynamicMesh) (Variables|Default|Get⚙%20Safe%20Normal%20Tolerance) false true)
  (Class|DynamicMeshComponent|ConfigureMaterialSet (Variables|Default|GetDynamicMeshComponent) (Utilities|Array|MakeArray (Variables|Default|Get🎨%20Material%20Trim) (Variables|Default|Get🎨%20Material%20Center)))
  (DynamicMeshActor|ReleaseAllComputeMeshes)
  (Transformation|AddWorldOffset (Variables|Default|GetDynamicMeshComponent) (Variables|Default|Get⚙%20Floor%20Location%20Offset) false false))

(fn ConstructionScript
  (|CallParentFunction)
  (CallFunction|UpdateUI)
  (CallFunction|UpdateUIEvent))

(fn FnBevel
  (params (TargetMesh :type Dynamic%20Mesh%20Object%20Reference) (Options%20Bevel%20Distance :type Float%20%28double-precision%29))
  (bind _returnvalue (Class|GeometryScriptLibraryMeshPolygroupFunctions|ComputePolygroupsfromAngleThreshold :TargetMesh TargetMesh :CreaseAngle 25.0 :Debug 0))
  (bind _returnvalue_2 (Class|GeometryScriptLibraryMeshModelingFunctions|ApplyMeshPolygroupBevel _returnvalue (Utilities|Struct|MakeGeometryScriptMeshBevelOptions Options%20Bevel%20Distance true 0 false "(Min=(X=0.000000,Y=0.000000,Z=0.000000),Max=(X=0.000000,Y=0.000000,Z=0.000000),IsValid=0)" "0.000000,0.000000,0.000000|0.000000,0.000000,-0.000000|1.000000,1.000000,1.000000" true) 0))
  (bind _returnvalue_3 (Class|GeometryScriptLibraryMeshNormalsFunctions|ComputeSplitNormals _returnvalue_2 (Utilities|Struct|MakeGeometryScriptSplitNormalsOptions true 25.0 false "(bDefaultLayer=True,ExtendedLayerIndex=0)") (Utilities|Struct|MakeGeometryScriptCalculateNormalsOptions true true) 0))
  (return _returnvalue_3))

(fn ApplyMaterials
  (params (Materials :type Array%20of%20Material%20Interface%20Object%20References))
  (Variables|Default|Set🎨%20Material%20Trim (Utilities|Array|Get(acopy) Materials))
  (Variables|Default|Set🎨%20Material%20Center (Utilities|Array|Get(acopy) Materials 1))
  (Class|DynamicMeshComponent|ConfigureMaterialSet (Variables|Default|GetDynamicMeshComponent) (Utilities|Array|MakeArray (Variables|Default|Get🎨%20Material%20Trim) (Variables|Default|Get🎨%20Material%20Center)))
  (return))

(fn UpdateUI
  (bind _asbp_dimensions (Utilities|Casting|CastToBP_Dimensions (Variables|/Script/Engine.ChildActorComponent|GetChildActor (Variables|Default|GetBP%20Dimensions))))
  (Variables|Essentials|SetAs%20BP%20Dimensions _asbp_dimensions)
  (Utilities|FlowControl|Sequence
    (:then_0
      (Rendering|Components|TextRender|SetText (Variables|/Game/LevelDesigner/Blueprints/BP_Dimensions.BP_Dimensions_C|GetText%20X (Variables|Essentials|GetAs%20BP%20Dimensions)) (Utilities|Text|ToText(Float) (.x (Variables|Default|Get⚙%20Handle)) "HalfToEven")))
    (:then_1
      (Rendering|Components|TextRender|SetText (Variables|/Game/LevelDesigner/Blueprints/BP_Dimensions.BP_Dimensions_C|GetText%20Y (Variables|Essentials|GetAs%20BP%20Dimensions)) (Utilities|Text|ToText(Float) (.y (Variables|Default|Get⚙%20Handle)) "HalfToEven")))
    (:then_2
      (if (not (Variables|Default|GetOverride%20Dimension%20Z?))
        (Rendering|Components|TextRender|SetText (Variables|/Game/LevelDesigner/Blueprints/BP_Dimensions.BP_Dimensions_C|GetText%20Z (Variables|Essentials|GetAs%20BP%20Dimensions)) (Utilities|Text|ToText(Float) (.z (Variables|Default|Get⚙%20Handle)) "HalfToEven"))))))