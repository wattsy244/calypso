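; BP_CornerExtrude is a level design tool that procedurally generates a rounded corner mesh with Geometry Script, sized by a handle, radius and ceiling extrusion.
; On rebuild it boolean-unions a foot box, a 90-degree revolved polygon and a ceiling box.
; Optional mirror and polygroup bevel passes follow, then normal and degenerate-triangle cleanup and material assignment.
; ApplyMaterials stores the first supplied material, and ClearMaterials resets it.
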(event EventBeginPlay
  (|CallParentFunction) ; This node is disabled and will not be called.\nDrag off pins to build functionality.
)

(event EventClearMaterials
  (bind (_offsetx _offsetz _array) (|GetPolygonInfo))
  (bind _handle (Variables|Settings|GetHandle))
  (bind _handle_2 (Variables|Settings|GetHandle))
  (bind _radius (Variables|Settings|GetRadius))
  ;[1 1 1] CLEAR MATERIALS
  (Variables|Settings|SetMaterial 0)
  (Class|DynamicMeshComponent|ConfigureMaterialSet (Variables|Default|GetDynamicMeshComponent) (Utilities|Array|MakeArray (Variables|Settings|GetMaterial)))
  (DynamicMeshActor|ReleaseAllComputeMeshes)
  ;[1 1 1] Foot
  (bind _returnvalue (Class|GeometryScriptLibraryMeshPrimitiveFunctions|AppendBox :TargetMesh (stale Events|EventOnRebuildGeneratedMesh TargetMesh) :Transform (Math|Transform|MakeTransform (Math|Vector|MakeVector (/ (.x _handle_2) 2.0) (/ (.y _handle_2) 2.0) 0.0) "0, 0, 0" "1.000000,1.000000,1.000000") :DimensionX (.x _handle_2) :DimensionY (.y _handle_2) :DimensionZ (.z _handle_2) :Debug 0))
  ;[1 1 1] Corner Angle
  (bind _returnvalue_2 (DynamicMeshActor|AllocateComputeMesh))
  (bind _returnvalue_3 (Class|GeometryScriptLibraryMeshPrimitiveFunctions|AppendRevolvePolygon :TargetMesh _returnvalue_2 :Transform (Math|Transform|MakeTransform (Math|Vector|MakeVector _offsetx 0.0 _offsetz) "0.000000,180.000000,-90.000000" "1.000000,1.000000,1.000000") :PolygonVertices _array :RevolveOptions (Utilities|Struct|MakeGeometryScriptRevolveOptions 9e+01 0.0 false false 9e+01 false true) :Radius (Variables|Settings|GetRadius) :Debug 0))
  (bind _returnvalue_4 (GeometryScript|Booleans|ApplyMeshBoolean :TargetMesh _returnvalue :ToolMesh _returnvalue_3 :Operation "Union" :Debug 0))
  ;[1 1 1] Ceiling
  (bind _returnvalue_5 (DynamicMeshActor|AllocateComputeMesh))
  (bind _returnvalue_6 (Class|GeometryScriptLibraryMeshPrimitiveFunctions|AppendBox :TargetMesh _returnvalue_5 :Transform (Math|Transform|MakeTransform (Math|Vector|MakeVector (+ (.x _handle) _radius) (/ (.y _handle) 2.0) (|(((Thickness/2)+Height)+Rad) (.x _handle) (.z _handle) _radius)) "90.000000,270.000000,90.000000" "1.000000,1.000000,1.000000") :DimensionX (.x _handle) :DimensionY (.y _handle) :DimensionZ (Variables|Settings|GetExtrudeCeiling) :Debug 0))
  (bind _returnvalue_7 (GeometryScript|Booleans|ApplyMeshBoolean :TargetMesh _returnvalue_4 :ToolMesh _returnvalue_6 :Operation "Union" :Debug 0))
  (bind _returnvalue_8 (Class|GeometryScriptLibraryMeshNormalsFunctions|ComputeSplitNormals :TargetMesh _returnvalue_7 :SplitOptions (Utilities|Struct|MakeGeometryScriptSplitNormalsOptions true 25.0 false "(bDefaultLayer=True,ExtendedLayerIndex=0)") :Debug 0))
  (Variables|Default|SetDynamicMesh _returnvalue_8)
  (if (Variables|Settings|GetbMirror)
    ;[1 1 1] Mirror
    (bind _returnvalue_9 (Class|GeometryScriptLibraryMeshBooleanFunctions|ApplyMeshMirror (Variables|Default|GetDynamicMesh) (Math|Transform|MakeTransform (Math|Vector|MakeVector (+ (+ (.x (Variables|Settings|GetHandle)) (Variables|Settings|GetRadius) (Variables|Settings|GetExtrudeCeiling)) (Variables|Settings|GetMirrorOffset)) 0.0 0.0) "0,90.000000,90.000000" "1.000000,1.000000,1.000000") (Utilities|Struct|MakeGeometryScriptMeshMirrorOptions false true true) 0))
    (Variables|Default|SetDynamicMesh _returnvalue_9))
  (if (Variables|Settings|GetbBevels)
    ;[1 1 1] Bevel
    (bind _returnvalue_10 (Class|GeometryScriptLibraryMeshModelingFunctions|ApplyMeshPolygroupBevel (Variables|Default|GetDynamicMesh) (Utilities|Struct|MakeGeometryScriptMeshBevelOptions (Variables|Settings|GetBevel%20Distance) false 0 false "(Min=(X=0.000000,Y=0.000000,Z=0.000000),Max=(X=0.000000,Y=0.000000,Z=0.000000),IsValid=0)" "0.000000,0.000000,0.000000|0.000000,0.000000,-0.000000|1.000000,1.000000,1.000000" true) 0))
    (Variables|Default|SetDynamicMesh _returnvalue_10))
  ;[1 1 1] Clean Up and material
  (bind _returnvalue_11 (Class|GeometryScriptLibraryMeshNormalsFunctions|ComputeSplitNormals :TargetMesh (Variables|Default|GetDynamicMesh) :SplitOptions (Utilities|Struct|MakeGeometryScriptSplitNormalsOptions true 35.0 false "(bDefaultLayer=True,ExtendedLayerIndex=0)") :Debug 0))
  (CallFunction|CleanDegenerateTris _returnvalue_11 0.0005 false true)
  (Class|DynamicMeshComponent|ConfigureMaterialSet (Variables|Default|GetDynamicMeshComponent) (Utilities|Array|MakeArray (Variables|Settings|GetMaterial)))
  (DynamicMeshActor|ReleaseAllComputeMeshes))

(event Events|EventOnRebuildGeneratedMesh
  (params (TargetMesh :type Dynamic%20Mesh%20Object%20Reference))
  (bind (_offsetx _offsetz _array) (|GetPolygonInfo))
  (bind _handle (Variables|Settings|GetHandle))
  (bind _handle_2 (Variables|Settings|GetHandle))
  (bind _radius (Variables|Settings|GetRadius))
  ;[1 1 1] Foot
  (bind _returnvalue (Class|GeometryScriptLibraryMeshPrimitiveFunctions|AppendBox :TargetMesh TargetMesh :Transform (Math|Transform|MakeTransform (Math|Vector|MakeVector (/ (.x _handle_2) 2.0) (/ (.y _handle_2) 2.0) 0.0) "0, 0, 0" "1.000000,1.000000,1.000000") :DimensionX (.x _handle_2) :DimensionY (.y _handle_2) :DimensionZ (.z _handle_2) :Debug 0))
  ;[1 1 1] Corner Angle
  (bind _returnvalue_2 (DynamicMeshActor|AllocateComputeMesh))
  (bind _returnvalue_3 (Class|GeometryScriptLibraryMeshPrimitiveFunctions|AppendRevolvePolygon :TargetMesh _returnvalue_2 :Transform (Math|Transform|MakeTransform (Math|Vector|MakeVector _offsetx 0.0 _offsetz) "0.000000,180.000000,-90.000000" "1.000000,1.000000,1.000000") :PolygonVertices _array :RevolveOptions (Utilities|Struct|MakeGeometryScriptRevolveOptions 9e+01 0.0 false false 9e+01 false true) :Radius (Variables|Settings|GetRadius) :Debug 0))
  (bind _returnvalue_4 (GeometryScript|Booleans|ApplyMeshBoolean :TargetMesh _returnvalue :ToolMesh _returnvalue_3 :Operation "Union" :Debug 0))
  ;[1 1 1] Ceiling
  (bind _returnvalue_5 (DynamicMeshActor|AllocateComputeMesh))
  (bind _returnvalue_6 (Class|GeometryScriptLibraryMeshPrimitiveFunctions|AppendBox :TargetMesh _returnvalue_5 :Transform (Math|Transform|MakeTransform (Math|Vector|MakeVector (+ (.x _handle) _radius) (/ (.y _handle) 2.0) (|(((Thickness/2)+Height)+Rad) (.x _handle) (.z _handle) _radius)) "90.000000,270.000000,90.000000" "1.000000,1.000000,1.000000") :DimensionX (.x _handle) :DimensionY (.y _handle) :DimensionZ (Variables|Settings|GetExtrudeCeiling) :Debug 0))
  (bind _returnvalue_7 (GeometryScript|Booleans|ApplyMeshBoolean :TargetMesh _returnvalue_4 :ToolMesh _returnvalue_6 :Operation "Union" :Debug 0))
  (bind _returnvalue_8 (Class|GeometryScriptLibraryMeshNormalsFunctions|ComputeSplitNormals :TargetMesh _returnvalue_7 :SplitOptions (Utilities|Struct|MakeGeometryScriptSplitNormalsOptions true 25.0 false "(bDefaultLayer=True,ExtendedLayerIndex=0)") :Debug 0))
  (Variables|Default|SetDynamicMesh _returnvalue_8)
  (if (Variables|Settings|GetbMirror)
    ;[1 1 1] Mirror
    (bind _returnvalue_9 (Class|GeometryScriptLibraryMeshBooleanFunctions|ApplyMeshMirror (Variables|Default|GetDynamicMesh) (Math|Transform|MakeTransform (Math|Vector|MakeVector (+ (+ (.x (Variables|Settings|GetHandle)) (Variables|Settings|GetRadius) (Variables|Settings|GetExtrudeCeiling)) (Variables|Settings|GetMirrorOffset)) 0.0 0.0) "0,90.000000,90.000000" "1.000000,1.000000,1.000000") (Utilities|Struct|MakeGeometryScriptMeshMirrorOptions false true true) 0))
    (Variables|Default|SetDynamicMesh _returnvalue_9))
  (if (Variables|Settings|GetbBevels)
    ;[1 1 1] Bevel
    (bind _returnvalue_10 (Class|GeometryScriptLibraryMeshModelingFunctions|ApplyMeshPolygroupBevel (Variables|Default|GetDynamicMesh) (Utilities|Struct|MakeGeometryScriptMeshBevelOptions (Variables|Settings|GetBevel%20Distance) false 0 false "(Min=(X=0.000000,Y=0.000000,Z=0.000000),Max=(X=0.000000,Y=0.000000,Z=0.000000),IsValid=0)" "0.000000,0.000000,0.000000|0.000000,0.000000,-0.000000|1.000000,1.000000,1.000000" true) 0))
    (Variables|Default|SetDynamicMesh _returnvalue_10))
  ;[1 1 1] Clean Up and material
  (bind _returnvalue_11 (Class|GeometryScriptLibraryMeshNormalsFunctions|ComputeSplitNormals :TargetMesh (Variables|Default|GetDynamicMesh) :SplitOptions (Utilities|Struct|MakeGeometryScriptSplitNormalsOptions true 35.0 false "(bDefaultLayer=True,ExtendedLayerIndex=0)") :Debug 0))
  (CallFunction|CleanDegenerateTris _returnvalue_11 0.0005 false true)
  (Class|DynamicMeshComponent|ConfigureMaterialSet (Variables|Default|GetDynamicMeshComponent) (Utilities|Array|MakeArray (Variables|Settings|GetMaterial)))
  (DynamicMeshActor|ReleaseAllComputeMeshes))

(event EventTick
  (params (DeltaSeconds :type Float%20%28single-precision%29))
  (|CallParentFunction DeltaSeconds) ; This node is disabled and will not be called.\nDrag off pins to build functionality.
)

(fn ConstructionScript
  (|CallParentFunction))

(fn ApplyMaterials
  (params (Materials :type Array%20of%20Material%20Interface%20Object%20References))
  (Variables|Settings|SetMaterial (Utilities|Array|Get(acopy) Materials))
  (return))