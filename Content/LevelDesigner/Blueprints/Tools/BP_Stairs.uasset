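; Level-design tool that procedurally builds linear stairs with Geometry Script, sized from a Handle vector.
; On mesh rebuild, it appends steps using either an adaptive or fixed step count, with optional floating style and polygroup bevel.
; Optional simplified collision extrudes a triangle or stepped-offset side profile into convex hulls, or previews it in a debug material instead.
; Material can be applied or cleared; clearing also reruns the build logic.
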(event `self.ClearMaterials`
  (bind _num_steps (`self.Num Steps`))
  (bind (_handle_x _handle_y _handle_z) (`KismetMathLibrary.BreakVector` (`self.Handle`)))
  (bind (_handle_x_2 _handle_y_2 _handle_z_2) (`KismetMathLibrary.BreakVector` (`self.Handle`)))
  (bind _stepheight (`self.StepHeight`))
  (bind (_handle_x_3 _handle_y_3 _handle_z_3) (`KismetMathLibrary.BreakVector` (`self.Handle`)))
  (bind _offsetsimplifiedstep (`self.OffsetSimplifiedStep`))
  (bind (_handle_x_4 _handle_y_4 _handle_z_4) (`KismetMathLibrary.BreakVector` (`self.Handle`)))
  (bind _stepheight_2 (`self.StepHeight`))
  (bind _num_steps_2 (`self.Num Steps`))
  (bind (_handle_x_5 _handle_y_5 _handle_z_5) (`KismetMathLibrary.BreakVector` (`self.Handle`)))
  (bind (_handle_x_6 _handle_y_6 _handle_z_6) (`KismetMathLibrary.BreakVector` (`self.Handle`)))
  (bind _target_mesh (`self.Target Mesh`))
  (bind _floating (`self.Floating`))
  (bind _returnvalue (* _stepheight _offsetsimplifiedstep))
  (bind _returnvalue_2 (/ _handle_x_5 _num_steps_2))
  (bind _returnvalue_3 (`KismetMathLibrary.FTrunc` (/ _handle_x_2 _stepheight)))
  (bind _returnvalue_4 (`KismetMathLibrary.FTrunc` (/ _handle_x_4 _stepheight_2)))
  (bind _returnvalue_5 (* _stepheight _returnvalue_3))
  (bind _returnvalue_6 (- (* _returnvalue_2 _num_steps_2) (/ _returnvalue_2 2.0)))
  (bind _returnvalue_7 (* (/ _handle_z_2 _returnvalue_3) _offsetsimplifiedstep))
  ;[1 1 1] CLEAR MATERIALS
  (set `self.Material` null)
  (`DynamicMeshComponent.ConfigureMaterialSet` (`self.DynamicMeshComponent`) (`|MakeArray` (`self.Material`)))
  (switch `/Game/LevelDesigner/Demo/Data/Enums/Tools/E_StairConstructionType` (`self.Type`) :!label _label ; Decided between adaptive step number or Fixed step number
    (:`NewEnumerator0`
      ;[1 1 1] Generate the Stairs
      (bind _returnvalue_8 (`GeometryScriptLibrary_MeshPrimitiveFunctions.AppendLinearStairs` (stale `self.OnRebuildGeneratedMesh` TargetMesh) (struct) (`KismetMathLibrary.MakeTransform` (`KismetMathLibrary.MakeVector` 0.0 (/ _handle_y_4 2.0))) _handle_y_4 (/ _handle_z_4 _returnvalue_4) _stepheight_2 _returnvalue_4 _floating null))
      (set `self.Target Mesh` _returnvalue_8))
    (:`NewEnumerator1`
      (bind _returnvalue_9 (`GeometryScriptLibrary_MeshPrimitiveFunctions.AppendLinearStairs` (stale `self.OnRebuildGeneratedMesh` TargetMesh) (struct) (`KismetMathLibrary.MakeTransform` (`KismetMathLibrary.MakeVector` 0.0 (/ _handle_y 2.0))) _handle_y (/ _handle_z _num_steps) (/ _handle_x _num_steps) _num_steps _floating null))
      (set `self.Target Mesh` _returnvalue_9)))
  (if (`self.bBevel`)
    ;[1 1 1] Bevel
    (`GeometryScriptLibrary_MeshPolygroupFunctions.ComputePolygroupsFromAngleThreshold` _target_mesh (make `GeometryScriptGroupLayer` true) 25.0 2 null)
    (bind _returnvalue_10 (`GeometryScriptLibrary_MeshModelingFunctions.ApplyMeshPolygroupBevel` _target_mesh (make `GeometryScriptMeshBevelOptions` (`self.DistanceBevel`) true) null))
    (bind _returnvalue_11 (`GeometryScriptLibrary_MeshNormalsFunctions.ComputeSplitNormals` _returnvalue_10 (make `GeometryScriptSplitNormalsOptions` true 25.0) (make `GeometryScriptCalculateNormalsOptions` true) null))
    (set `self.Target Mesh` _returnvalue_11))
  (if (`self.bSimplifiedCollision`)
    ;[1 1 1] Simplified Collision Generation
    (bind _returnvalue_12 (`self.AllocateComputeMesh`))
    (set `self.Simplified` _returnvalue_12)
    (bind _returnvalue_13 (`GeometryScriptLibrary_MeshPrimitiveFunctions.AppendSimpleExtrudePolygon` (`self.Simplified`) (struct) (`KismetMathLibrary.MakeTransform` (0.0 0.0 0.0) (struct :`Pitch` 90.0 :`Roll` 90.0)) (select `bool` (`self.bTriangle`) :`false` (select `/Game/LevelDesigner/Demo/Data/Enums/Tools/E_StairConstructionType` (`self.Type`) :`NewEnumerator0` (`|MakeArray` (0.0 0.0) (`KismetMathLibrary.MakeVector2D` _returnvalue_7) (`KismetMathLibrary.MakeVector2D` _handle_z_3 (- _returnvalue_5 _returnvalue)) (`KismetMathLibrary.MakeVector2D` _handle_z_3 _returnvalue_5) (`KismetMathLibrary.MakeVector2D` 0.0 _returnvalue_5) :!type "Vector2D Structure") :`NewEnumerator1` (`|MakeArray` (0.0 0.0) (`KismetMathLibrary.MakeVector2D` _returnvalue_7) (`KismetMathLibrary.MakeVector2D` _handle_z_3 (- _handle_x_3 _returnvalue)) (`KismetMathLibrary.MakeVector2D` _handle_z_3 _handle_x_3) (`KismetMathLibrary.MakeVector2D` 0.0 _handle_x_3) :!type "Vector2D Structure")) :`true` (select `/Game/LevelDesigner/Demo/Data/Enums/Tools/E_StairConstructionType` (`self.Type`) :`NewEnumerator0` (`|MakeArray` (0.0 0.0) (`KismetMathLibrary.MakeVector2D` _handle_z_6 _returnvalue_6) (`KismetMathLibrary.MakeVector2D` 0.0 _returnvalue_6) :!type "Vector2D Structure") :`NewEnumerator1` (`|MakeArray` (0.0 0.0) (`KismetMathLibrary.MakeVector2D` _handle_z_6 _handle_x_6) (`KismetMathLibrary.MakeVector2D` 0.0 _handle_x_6) :!type "Vector2D Structure"))) _handle_y_3 0 true "Base" null))
    (set `self.Simplified` _returnvalue_13)
    (if (`self.bPreviewSimplified(turnOFFBEFOREBAKE)`)
      ;;[1 1 1] This is just to preview temporary the Collision Mesh
      (bind _returnvalue_14 (`GeometryScriptLibrary_MeshMaterialFunctions.RemapMaterialIDs` (`self.Simplified`) 0 1 null))
      (bind _returnvalue_15 (`GeometryScriptLibrary_MeshBasicEditFunctions.AppendMesh` (`self.Target Mesh`) _returnvalue_14 (struct) false null))
      (set `self.Target Mesh` _returnvalue_15)
      (else
        (bind _returnvalue_16 (`GeometryScriptLibrary_CollisionFunctions.SetDynamicMeshCollisionFromMesh` (`self.Simplified`) (`self.DynamicMeshComponent`) (make `GeometryScriptCollisionFromMeshOptions` false "ConvexHulls" false false false 1.0 false 25 0.1 "Z" false) null))
        (set `self.Target Mesh` _returnvalue_16)))
    (else
      ;[1 1 1] Don't simplified the Collision
      (`GeometryScriptLibrary_CollisionFunctions.ResetDynamicMeshCollision` (`self.DynamicMeshComponent`) false null)))
  ;[1 1 1] Apply Material
  (`DynamicMeshComponent.ConfigureMaterialSet` (`self.DynamicMeshComponent`) (`|MakeArray` (`self.Material`) "/Game/LevelDesigner/Demo/Materials/M_DebugTool.M_DebugTool"))
  (`self.CleanDegenerateTris` (`self.Target Mesh`))
  (`self.ReleaseAllComputeMeshes`))

(event `self.OnRebuildGeneratedMesh`
  (params (TargetMesh :type "DynamicMesh Object Reference"))
  (goto _label))

(fn `ApplyMaterials`
  (params (Materials :type "Array of MaterialInterface Object Reference (by ref)"))
  (set `self.Material` (`|GetArrayItem` Materials))
  (return))

(fn `UserConstructionScript`
  (`parent.UserConstructionScript`))