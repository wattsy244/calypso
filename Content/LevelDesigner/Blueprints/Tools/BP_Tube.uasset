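; Level-design tool actor that procedurally builds a tube or curved wall with Geometry Script when its generated mesh rebuilds.
; A rectangular thickness-by-height profile is revolved, optionally beveled, then optionally repeated as gapped segments around the arc.
; An extruded rounded-rectangle window cutter, optionally repeated, is boolean-subtracted, or unioned with a debug material to preview it.
; Split normals, degenerate-triangle cleanup and material assignment finish the mesh.
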(event EventBeginPlay
  (|CallParentFunction))

(event EventClearMaterials
  ;[1 1 1] CLEAR MATERIALS
  (Variables|Settings|RevolveOptions|SetMaterial 0)
  ;[1 1 1] Create Tube
  (bind _returnvalue (Class|GeometryScriptLibraryMeshPrimitiveFunctions|AppendRevolvePolygon :TargetMesh (Variables|Default|GetDynamicMesh) :PolygonVertices (|MakePolygonVertices) :RevolveOptions (|GetRevolveOptions) :Radius (|GetRadius) :Steps (Variables|Settings|RevolveOptions|GetSteps) :Debug 0))
  (Variables|Default|SetDynamicMesh _returnvalue)
  (if (Variables|Settings|Bevels|GetbBevel)
    ;[1 1 1] Bevel
    (bind _returnvalue_2 (Class|GeometryScriptLibraryMeshModelingFunctions|ApplyMeshPolygroupBevel (Variables|Default|GetDynamicMesh) (Utilities|Struct|MakeGeometryScriptMeshBevelOptions (Variables|Settings|Bevels|GetBevelDistance) false 0 false "(Min=(X=0.000000,Y=0.000000,Z=0.000000),Max=(X=0.000000,Y=0.000000,Z=0.000000),IsValid=0)" "0.000000,0.000000,0.000000|0.000000,0.000000,-0.000000|1.000000,1.000000,1.000000" true) 0))
    (Variables|Default|SetDynamicMesh _returnvalue_2))
  (Utilities|McRepeater)
  (DynamicMeshActor|ReleaseAllComputeMeshes)
  (if (Variables|Settings|Window|GetbWindow)
    (Utilities|McWindowCutter))
  ;[1 1 1] This helps smoothing the Normals
  (bind _returnvalue_3 (Class|GeometryScriptLibraryMeshNormalsFunctions|ComputeSplitNormals :TargetMesh (Variables|Default|GetDynamicMesh) :SplitOptions (Utilities|Struct|MakeGeometryScriptSplitNormalsOptions true 45.0 false "(bDefaultLayer=True,ExtendedLayerIndex=0)") :Debug 0))
  ;[1 1 1] Apply Materials
  (CallFunction|CleanDegenerateTris _returnvalue_3 0.0005 false true)
  (Class|DynamicMeshComponent|ConfigureMaterialSet (Variables|Default|GetDynamicMeshComponent) (Utilities|Array|MakeArray (Variables|Settings|RevolveOptions|GetMaterial) "/Game/LevelDesigner/Demo/Materials/M_DebugTool.M_DebugTool")))

(event Events|EventOnRebuildGeneratedMesh
  (params (TargetMesh :type Dynamic%20Mesh%20Object%20Reference))
  (Variables|Default|SetDynamicMesh TargetMesh)
  ;[1 1 1] Create Tube
  (bind _returnvalue (Class|GeometryScriptLibraryMeshPrimitiveFunctions|AppendRevolvePolygon :TargetMesh (Variables|Default|GetDynamicMesh) :PolygonVertices (|MakePolygonVertices) :RevolveOptions (|GetRevolveOptions) :Radius (|GetRadius) :Steps (Variables|Settings|RevolveOptions|GetSteps) :Debug 0))
  (Variables|Default|SetDynamicMesh _returnvalue)
  (if (Variables|Settings|Bevels|GetbBevel)
    ;[1 1 1] Bevel
    (bind _returnvalue_2 (Class|GeometryScriptLibraryMeshModelingFunctions|ApplyMeshPolygroupBevel (Variables|Default|GetDynamicMesh) (Utilities|Struct|MakeGeometryScriptMeshBevelOptions (Variables|Settings|Bevels|GetBevelDistance) false 0 false "(Min=(X=0.000000,Y=0.000000,Z=0.000000),Max=(X=0.000000,Y=0.000000,Z=0.000000),IsValid=0)" "0.000000,0.000000,0.000000|0.000000,0.000000,-0.000000|1.000000,1.000000,1.000000" true) 0))
    (Variables|Default|SetDynamicMesh _returnvalue_2))
  (Utilities|McRepeater)
  (DynamicMeshActor|ReleaseAllComputeMeshes)
  (if (Variables|Settings|Window|GetbWindow)
    (Utilities|McWindowCutter))
  ;[1 1 1] This helps smoothing the Normals
  (bind _returnvalue_3 (Class|GeometryScriptLibraryMeshNormalsFunctions|ComputeSplitNormals :TargetMesh (Variables|Default|GetDynamicMesh) :SplitOptions (Utilities|Struct|MakeGeometryScriptSplitNormalsOptions true 45.0 false "(bDefaultLayer=True,ExtendedLayerIndex=0)") :Debug 0))
  ;[1 1 1] Apply Materials
  (CallFunction|CleanDegenerateTris _returnvalue_3 0.0005 false true)
  (Class|DynamicMeshComponent|ConfigureMaterialSet (Variables|Default|GetDynamicMeshComponent) (Utilities|Array|MakeArray (Variables|Settings|RevolveOptions|GetMaterial) "/Game/LevelDesigner/Demo/Materials/M_DebugTool.M_DebugTool")))

(fn ConstructionScript
  (|CallParentFunction))

(fn FnRepeater
  (params (InputPin :type Dynamic%20Mesh%20Object%20Reference) (Instances :type Integer))
  (bind _returnvalue (DynamicMeshActor|AllocateComputeMesh))
  (bind _copytomeshout (GeometryScript|Decomposition|CopyMeshtoMesh InputPin _returnvalue 0))
  (bind _returnvalue_2 (Class|GeometryScriptLibraryMeshBasicEditFunctions|AppendMeshRepeated InputPin _copytomeshout (Math|Transform|MakeTransform "0, 0, 0" (Math|Rotator|MakeRotator 0.0 0.0 (|GetRotationRate)) "1.000000,1.000000,1.000000") (- Instances 1) true false 0))
  (return _returnvalue_2))

(fn ApplyMaterials
  (params (Materials :type Array%20of%20Material%20Interface%20Object%20References))
  (Variables|Settings|RevolveOptions|SetMaterial (Utilities|Array|Get(acopy) Materials))
  (return))