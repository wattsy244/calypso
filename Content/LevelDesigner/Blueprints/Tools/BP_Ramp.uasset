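; BP_Ramp is a level design tool that generates a ramp as a dynamic mesh with complex-as-simple collision.
; On rebuild, it resets the mesh, builds a four-sided profile from TopPoint and FloorPoint, extrudes it by TopPoint.Y and cleans degenerate triangles.
; Each rebuild also adds a 180-degree relative rotation to the mesh component and applies Material.
; ClearMaterials nulls Material, then runs the same rebuild.
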(event `self.ClearMaterials`
  (bind (_toppoint_x _toppoint_y _toppoint_z) (`KismetMathLibrary.BreakVector` (`self.TopPoint`)))
  (bind _floorpoint_x (`KismetMathLibrary.BreakVector` (`self.FloorPoint`)))
  ;[1 1 1] CLEAR MATERIALS
  (set `self.Material` null)
  (`DynamicMeshComponent.ConfigureMaterialSet` (`self.DynamicMeshComponent`) (`|MakeArray` (`self.Material`)))
  (bind _returnvalue (`BaseDynamicMeshComponent.GetDynamicMesh` (`self.DynamicMeshComponent`) :!label _label))
  (bind _returnvalue_2 (`DynamicMesh.Reset` _returnvalue))
  (`SceneComponent.K2_AddRelativeRotation` (`self.DynamicMeshComponent`) (struct :`Yaw` 180.0) false false)
  (bind _returnvalue_3 (`GeometryScriptLibrary_MeshPrimitiveFunctions.AppendTriangulatedPolygon` _returnvalue_2 (struct) (`KismetMathLibrary.MakeTransform` (`KismetMathLibrary.MakeVector` 0.0 0.0 _toppoint_z) (struct :`Roll` 90.0)) (`|MakeArray` (0.0 0.0) (`KismetMathLibrary.MakeVector2D` 0.0 _toppoint_z) (`KismetMathLibrary.MakeVector2D` _floorpoint_x _toppoint_z) (`KismetMathLibrary.MakeVector2D` _toppoint_x) :!type "Vector2D Structure") false null))
  (bind _returnvalue_4 (`GeometryScriptLibrary_MeshModelingFunctions.ApplyMeshExtrude` _returnvalue_3 (make `GeometryScriptMeshExtrudeOptions` _toppoint_y (0.0 1.0 0.0)) null))
  (`self.CleanDegenerateTris` _returnvalue_4)
  (`DynamicMeshComponent.ConfigureMaterialSet` (`self.DynamicMeshComponent`) (`|MakeArray` (`self.Material`)))
  (`self.ReleaseAllComputeMeshes`)
  (`DynamicMeshComponent.EnableComplexAsSimpleCollision` (`self.DynamicMeshComponent`)))

(event `self.OnRebuildGeneratedMesh`
  (params (TargetMesh :type "DynamicMesh Object Reference"))
  (goto _label))

(fn `UserConstructionScript`
  (`parent.UserConstructionScript`))