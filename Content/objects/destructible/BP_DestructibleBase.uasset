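; Base destructible object Blueprint that loses HP through an Impact event carrying a damage amount.
; When HP reaches zero or below, it spawns the NS_Brick effect at coordinates from a setup graph, which contains a vertical offset from the actor's location.
; Instead of destroying itself, the actor then teleports far below the world to disappear.
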(event `/Game/temporarykieranstuff/BPI_ProjectileNew.Impact`
  (params (Damage :type Integer))
  (bind (_returnvalue_x _returnvalue_y _returnvalue_z) (`KismetMathLibrary.BreakVector` (`self.K2_GetActorLocation`)))
  (bind _output_get (set `self.HP` (- (`self.HP`) Damage)))
  (if (<= _output_get 0)
    (`NiagaraFunctionLibrary.SpawnSystemAtLocation` "/Game/playerlogic/particle/NS_Brick.NS_Brick" (`KismetMathLibrary.MakeVector` _returnvalue_x _returnvalue_y (+ _returnvalue_z 45.0)))
    (`self.K2_SetActorLocation` (0.0 0.0 -999999.0))))

(fn `UserConstructionScript`)