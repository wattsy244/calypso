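; Helper actor that displays a coloured damage indicator through its Damageindicator widget component.
; On BeginPlay it casts the widget to UI_DamageIndicatorTemporary, then applies Colour to the Value text and fills it via Remove Comma.
; The input to Remove Comma is hardcoded, with no real damage value passed in.
; That helper's graph holds a random-integer-to-text chain that strips commas.
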(event `self.ReceiveBeginPlay`
  (bind _asui_damage_indicator_temporary (cast `/Game/temporarykieranstuff/UI_DamageIndicatorTemporary` (`WidgetComponent.GetWidget` (`self.damageindicator`))))
  (bind _value (`/Game/temporarykieranstuff/UI_DamageIndicatorTemporary.value` _asui_damage_indicator_temporary))
  (`TextBlock.SetColorAndOpacity` _value (make `SlateColor` (`self.colour`)))
  (set `TextBlock.Text` (`KismetTextLibrary.Conv_StringToText` (`KismetStringLibrary.Replace` (`KismetStringLibrary.Conv_IntToString` (`KismetMathLibrary.RandomInteger` 3)) ",")) _value))

(fn `UserConstructionScript`)