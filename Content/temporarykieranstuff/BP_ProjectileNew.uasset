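; BP_ProjectileNew is a projectile that reports impacts and leaves a damage indicator in the firing player's colour.
; On collision, targets tagged Enemy are cast to BP_TwinStickNPC for a projectile impact message.
; Those NPCs and all untagged actors receive a fixed-value impact message, then it spawns BP_DamageIndicatorHelperActor and destroys itself.
; The colour comes from the GameInstance via the instigator's controller ID, while GetColour is an unused black stub.
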(event `self.col.OnComponentHit`
  (params (HitComponent :type "PrimitiveComponent Object Reference") (OtherActor :type "Actor Object Reference") (OtherComp :type "PrimitiveComponent Object Reference") (NormalImpulse :type "Vector Structure") (Hit :type "HitResult Structure (by ref)"))
  (if (`self.ActorHasTag` OtherActor "Enemy")
    (bind _asbp_twin_stick_npc (cast `/Game/Variant_TwinStick/Blueprints/AI/BP_TwinStickNPC` OtherActor))
    (message `/Game/Variant_TwinStick/Blueprints/BPI_Twinstick.ProjectileImpact` _asbp_twin_stick_npc (0.0 0.0 0.0)))
  (message `/Game/temporarykieranstuff/BPI_ProjectileNew.Impact` OtherActor 250)
  (`|SpawnActorFromClass` "/Game/temporarykieranstuff/BP_DamageIndicatorHelperActor.BP_DamageIndicatorHelperActor_C" (`KismetMathLibrary.MakeTransform` (`self.K2_GetActorLocation`)) "AlwaysSpawn" "MultiplyWithRoot" null 0 (`self.getMyColour`) null)
  (`self.K2_DestroyActor`))

(fn `getColour`
  (params (myindex :type Integer))
  (returns (colour :type "LinearColor Structure"))
  (return))

(fn `getMyColour`
  (returns (colour :type "LinearColor Structure"))
  (bind _asplayer_controller (cast `PlayerController` (`self.GetInstigatorController`)))
  (bind _colour (message `/Game/temporarykieranstuff/BPI_Instance.getColour` (`GameplayStatics.GetGameInstance`) (`GameplayStatics.GetPlayerControllerID` _asplayer_controller)))
  (return _colour))

(fn `UserConstructionScript`)