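; Selection screen actor that displays four meshes as spinning models, presumably for player selection.
; On BeginPlay it registers itself with the game mode through an interface message and fills its mesh array.
; An interface event toggles an indexed mesh's visibility and optionally shifts the whole actor by a given vector.
; Tick rotates every mesh by a fixed per-frame step; the player-info interface functions are empty stubs.
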(event `self.ReceiveBeginPlay`
  (message `/Game/selectionlogic/BPI_SelectionInterface.BPI_SetSelectionActor` (`GameplayStatics.GetGameMode`) self)
  (set `self.meshes` (`|MakeArray` (`self.0`) (`self.1`) (`self.2`) (`self.3`))))

(event `/Game/selectionlogic/BPI_SelectionInterface.BPI_ManipulateSelectionActor`
  (params (index :type Integer) (shift :type Boolean) (vector :type "Vector Structure"))
  (bind _output (`|GetArrayItem` (`self.meshes`) index))
  (`SceneComponent.SetVisibility` _output (not (`SceneComponent.bVisible` _output)) false)
  (if shift
    (`self.K2_AddActorWorldOffset` vector)))

(event `self.ReceiveTick`
  (params (DeltaSeconds :type "Float (single-precision)"))
  (for _array_element (`self.meshes`)
    (`SceneComponent.K2_AddLocalRotation` _array_element (struct :`Yaw` 1.0) false false)))

(fn `BPI_GetAllPlayerInfo`
  (returns (info :type "Map of Integer to /Game/playerlogicbetter/characterclassinfo/STRUCT_PlayerInfo Structure"))
  (return))

(fn `BPI_GetPlayerInfo`
  (params (index :type Integer))
  (returns (info :type "/Game/playerlogicbetter/characterclassinfo/STRUCT_PlayerInfo Structure"))
  (return))

(fn `BPI_IsPlayerRegistered`
  (returns (registered :type Boolean))
  (return false))

(fn `UserConstructionScript`)