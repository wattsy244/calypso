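; Player controller for a local multiplayer twin-stick shooter that registers players and drives their characters.
; Player 0 registers on BeginPlay and others on any key press, saving state to the GameInstance through interface messages.
; Initialise adds the control scheme's mapping context, then spawns and possesses a CH_PlayerBase for registered players.
; Mouse or stick rotates the mesh to aim, cooldown-gated attacks spawn projectiles, and a timer prints debug status.
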(event `self.ReceiveBeginPlay`
  (if (== (`GameplayStatics.GetPlayerControllerID` self) 0)
    (`self.registerPlayer`)))

(event `Key|AnyKey`
  (params (Key :type "Key Structure"))
  (:`Pressed`
    (message `/Game/selectionlogic/BPI_SelectionInterface.BPI_AddUser` (`GameplayStatics.GetGameMode`) self)
    (`self.registerPlayer`)))

(event `Initialise`
  (bind _info_controlscheme (break `/Game/playerlogicbetter/characterclassinfo/STRUCT_PlayerInfo` (`self.getPlayerInfo`)))
  (bind _info_controlscheme_2 (break `/Game/playerlogicbetter/characterclassinfo/STRUCT_PlayerInfo` (`self.getPlayerInfo`)))
  (`/Engine/EditorBlueprintResources/StandardMacros.IsValid` (`self.owningCharacter`)
    (:`Is Not Valid`
      (`self.setUpPlayerInfo`)
      (`EnhancedInputSubsystemInterface.AddMappingContext` (subsystem `EnhancedInputLocalPlayerSubsystem`) (select `/Game/playerlogicbetter/characterclassinfo/ENUM_ControlScheme` _info_controlscheme_2 :`NewEnumerator0` "/Game/playerlogicbetter/input/IAC_PlayerMainKeyboard.IAC_PlayerMainKeyboard" :`NewEnumerator1` "/Game/playerlogicbetter/input/IAC_PlayerMainController.IAC_PlayerMainController" :!type "InputMappingContext Object Reference") 0 (struct))
      (`KismetSystemLibrary.K2_SetTimerDelegate` (delegate `debugchecks`) 5.0 true)
      (if (`self.registered`)
        (bind _returnvalue (`|SpawnActorFromClass` "/Game/playerlogicbetter/CH_PlayerBase.CH_PlayerBase_C" (`KismetMathLibrary.MakeTransform` (0.0 0.0 92.0)) "Undefined" "MultiplyWithRoot" null null))
        (bind _output_get (set `self.owningCharacter` _returnvalue))
        (`self.Possess` _output_get)
        (switch `/Game/playerlogicbetter/characterclassinfo/ENUM_ControlScheme` _info_controlscheme
          (:`NewEnumerator0`
            (`KismetSystemLibrary.K2_SetTimer` null "lookAtMouse" 0.01 true true)
            (set `self.bShowMouseCursor` true)))))))

(event `debugchecks`
  (`/Engine/EditorBlueprintResources/StandardMacros.IsValid` (`self.owningCharacter`)
    (:`Is Valid`
      (`KismetSystemLibrary.PrintString` (`KismetStringLibrary.Concat_StrStr` (`KismetStringLibrary.Concat_StrStr` "PLAYER " (`KismetStringLibrary.Conv_IntToString` (+ (`GameplayStatics.GetPlayerControllerID` self) 1))) "  is registered and has a character!") true true (struct :`R` 0.325197 :`G` 1.0 :`A` 1.0) 3.0))
    (:`Is Not Valid`
      (`KismetSystemLibrary.PrintString` (`KismetStringLibrary.Concat_StrStr` (`KismetStringLibrary.Concat_StrStr` "PLAYER " (`KismetStringLibrary.Conv_IntToString` (+ (`GameplayStatics.GetPlayerControllerID` self) 1))) "  HAS NO PLAYER CHARACTER !! NORMAL IF ON SELECTION SCREEN") true true (struct :`R` 1.0 :`G` 0.025545 :`A` 1.0) 3.0))))

(event `EnhancedInput|/Game/playerlogicbetter/input/IA_MoveNew`
  (params (ActionValue :type "Vector2D Structure") (ElapsedSeconds :type "Float (double-precision)") (TriggeredSeconds :type "Float (double-precision)") (InputAction :type "InputAction Object Reference" :default "/Game/playerlogicbetter/input/IA_MoveNew.IA_MoveNew"))
  (:`Triggered`
    (`Pawn.AddMovementInput` (`self.owningCharacter`) (`self.GetActorForwardVector` (`self.owningCharacter`)) ActionValue_X false)
    (`Pawn.AddMovementInput` (`self.owningCharacter`) (`self.GetActorRightVector` (`self.owningCharacter`)) ActionValue_Y false)))

(event `EnhancedInput|/Game/playerlogicbetter/input/IA_AttackNew`
  (params (ActionValue :type Boolean) (ElapsedSeconds :type "Float (double-precision)") (TriggeredSeconds :type "Float (double-precision)") (InputAction :type "InputAction Object Reference" :default "/Game/playerlogicbetter/input/IA_AttackNew.IA_AttackNew"))
  (bind _info_controlscheme (break `/Game/playerlogicbetter/characterclassinfo/STRUCT_PlayerInfo` (`self.getPlayerInfo`)))
  (bind _mesh (`Character.Mesh` (`self.owningCharacter`)))
  (bind (_returnvalue_roll _returnvalue_pitch _returnvalue_yaw) (`KismetMathLibrary.BreakRotator` (`SceneComponent.K2_GetComponentRotation` _mesh)))
  (:`Triggered`
    (`self.cooldown` 0.1 :!label _label
      (:`immediate`
        (`|SpawnActorFromClass` "/Game/temporarykieranstuff/BP_ProjectileNew.BP_ProjectileNew_C" (`KismetMathLibrary.MakeTransform` (`SceneComponent.K2_GetComponentLocation` _mesh) (`KismetMathLibrary.MakeRotator` 0.0 0.0 (- _returnvalue_yaw 279.0))) "Undefined" "MultiplyWithRoot" null (`GameplayStatics.GetPlayerControllerID` self) null)
        (switch `/Game/playerlogicbetter/characterclassinfo/ENUM_ControlScheme` _info_controlscheme
          (:`NewEnumerator1`
            (`self.PlayDynamicForceFeedback` 0.1 0.1)))))))

(event `Key|LeftMouseButton`
  (params (Key :type "Key Structure"))
  (:`Pressed`
    (goto _label)))

(event `EnhancedInput|/Game/playerlogicbetter/input/IA_AimControllerNew`
  (params (ActionValue :type "Vector2D Structure") (ElapsedSeconds :type "Float (double-precision)") (TriggeredSeconds :type "Float (double-precision)") (InputAction :type "InputAction Object Reference" :default "/Game/playerlogicbetter/input/IA_AimControllerNew.IA_AimControllerNew"))
  (:`Triggered`
    (`SceneComponent.K2_SetRelativeRotation` (`Character.Mesh` (`self.owningCharacter`)) (`KismetMathLibrary.Conv_VectorToRotator` (`KismetMathLibrary.MakeVector` ActionValue_Y ActionValue_X)) false false)))

(fn `getPlayerInfo`
  (returns (info :type "/Game/playerlogicbetter/characterclassinfo/STRUCT_PlayerInfo Structure"))
  (bind _info (message `/Game/selectionlogic/BPI_SelectionInterface.BPI_GetPlayerInfo` (`GameplayStatics.GetGameInstance`) (`GameplayStatics.GetPlayerControllerID` self)))
  (return _info))

(fn `lookAtMouse`
  (bind (_returnvalue_roll _returnvalue_pitch _returnvalue_yaw) (`KismetMathLibrary.BreakRotator` (`KismetMathLibrary.FindLookAtRotation` (`.Location` (`GameplayStatics.BreakHitResult` (`self.GetHitResultUnderCursorByChannel` "TraceTypeQuery1"))) (`self.K2_GetActorLocation` (`self.K2_GetPawn`)))))
  (if (`self.registered`)
    (`SceneComponent.K2_SetWorldRotation` (`Character.Mesh` (`self.owningCharacter`)) (`KismetMathLibrary.MakeRotator` _returnvalue_roll _returnvalue_pitch (+ 90.0 _returnvalue_yaw)) false false)))

(fn `registerPlayer`
  (set `self.registered` true)
  (bind _structout (setmembers `/Game/playerlogicbetter/characterclassinfo/STRUCT_PlayerInfo` :`StructRef` (`self.getPlayerInfo`) :`Registered` true))
  (`self.updatePlayerInfo` _structout))

(fn `setUpPlayerInfo`
  (bind _output_get (set `self.playerInfo` (`self.getPlayerInfo`)))
  (set `self.registered` (`.Registered_7_DD5B6DE14DF04C889E7A258E8FEBCD2F` (break `/Game/playerlogicbetter/characterclassinfo/STRUCT_PlayerInfo` _output_get))))

(fn `updatePlayerInfo`
  (params (In :type "/Game/playerlogicbetter/characterclassinfo/STRUCT_PlayerInfo Structure"))
  (message `/Game/selectionlogic/BPI_SelectionInterface.BPI_UpdatePlayerInfo` (`GameplayStatics.GetGameInstance`) (`GameplayStatics.GetPlayerControllerID` self) In))

(fn `UserConstructionScript`)