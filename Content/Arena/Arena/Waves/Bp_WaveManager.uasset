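; Wave manager Blueprint for the arena mode that sets the enemy cap and round type for each wave through GMB_MainGame.
; It reads the wave index from the game mode on BeginPlay, then NextWave increments it and picks a standard or mini-boss wave.
; Both write back the index and an NPC cap scaled by wave number.
; Hard-coded milestone waves flag a boss round with extra enemies; the flag is never cleared here.
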(event `self.ReceiveBeginPlay`
  ; Get wave
  (bind _asgmb_main_game (cast `/Game/playerlogic/GMB_MainGame` (`GameplayStatics.GetGameMode`)))
  (set `self.CurrentWave` (`/Game/playerlogic/GMB_MainGame.wave index` _asgmb_main_game)))

(event `StartWave`
  ; Standard wave
  (`KismetSystemLibrary.PrintString` (`KismetStringLibrary.Conv_IntToString` (`self.CurrentWave`)))
  (bind _asgmb_main_game (cast `/Game/playerlogic/GMB_MainGame` (`GameplayStatics.GetGameMode`)))
  (set `/Game/playerlogic/GMB_MainGame.Max NPC Cap` (* (`self.EnemiesPerWave`) (`self.CurrentWave`)) _asgmb_main_game)
  (bind _output_get (set `/Game/playerlogic/GMB_MainGame.wave index` (`self.CurrentWave`) _asgmb_main_game)))

(event `NextWave`
  ; Next round checker
  (bind _result (`/Engine/EditorBlueprintResources/StandardMacros.IncrementInt` (`self.CurrentWave`))
    (:`  `
      (`KismetSystemLibrary.PrintString` (`KismetStringLibrary.Conv_IntToString` _result))
      (if (== (`self.CurrentWave`) 5)
        (`self.mini boss`)
        (elif (== (`self.CurrentWave`) 10)
          (`self.mini boss`)
          (elif (== (`self.CurrentWave`) 15)
            (`self.mini boss`)
            (else
              (`self.StartWave`))))))))

(event `mini boss`
  ; Boss wave going to change to mini boss
  (bind _asgmb_main_game (cast `/Game/playerlogic/GMB_MainGame` (`GameplayStatics.GetGameMode`)))
  (set `/Game/playerlogic/GMB_MainGame.Boss round` true _asgmb_main_game)
  (set `/Game/playerlogic/GMB_MainGame.Max NPC Cap` (+ (* (`self.EnemiesPerWave`) (`self.CurrentWave`)) 10) _asgmb_main_game)
  (set `/Game/playerlogic/GMB_MainGame.wave index` (`self.CurrentWave`) _asgmb_main_game))

(fn `UserConstructionScript`)