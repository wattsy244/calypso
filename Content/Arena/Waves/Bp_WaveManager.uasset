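; Wave manager for the twin-stick arena that sets the NPC cap and boss state for each round through BP_TwinStickGameMode.
; It reads the starting wave from the game mode on BeginPlay, and NextWave increments it before choosing a standard or boss wave.
; Both wave types scale the cap by wave number and write the index back.
; Only wave five triggers the boss round, which raises the per-wave count and sets BossRound.
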(event `self.ReceiveBeginPlay`
  ; Get wave
  (bind _asbp_twin_stick_game_mode (cast `/Game/Variant_TwinStick/Blueprints/BP_TwinStickGameMode` (`GameplayStatics.GetGameMode`)))
  (set `self.CurrentWave` (`/Game/Variant_TwinStick/Blueprints/BP_TwinStickGameMode.Wave Index` _asbp_twin_stick_game_mode)))

(event `StartWave`
  ; Standard wave
  (bind _asbp_twin_stick_game_mode (cast `/Game/Variant_TwinStick/Blueprints/BP_TwinStickGameMode` (`GameplayStatics.GetGameMode`)))
  (set `/Game/Variant_TwinStick/Blueprints/BP_TwinStickGameMode.Max NPC Cap` (* (`self.EnemiesPerWave`) (`self.CurrentWave`)) _asbp_twin_stick_game_mode)
  (bind _output_get (set `/Game/Variant_TwinStick/Blueprints/BP_TwinStickGameMode.Wave Index` (`self.CurrentWave`) _asbp_twin_stick_game_mode))
  (`KismetSystemLibrary.PrintString` (`KismetStringLibrary.Conv_IntToString` _output_get)))

(event `NextWave`
  ; Next round checker
  (`/Engine/EditorBlueprintResources/StandardMacros.IncrementInt` (`self.CurrentWave`)
    (:`  `
      (if (== (`self.CurrentWave`) 5)
        (`self.Boss`)
        (else
          (`self.StartWave`))))))

(event `Boss`
  ; Boss wave
  (bind _asbp_twin_stick_game_mode (cast `/Game/Variant_TwinStick/Blueprints/BP_TwinStickGameMode` (`GameplayStatics.GetGameMode`)))
  (set `/Game/Variant_TwinStick/Blueprints/BP_TwinStickGameMode.Max NPC Cap` (* (+ (`self.EnemiesPerWave`) 10) (`self.CurrentWave`)) _asbp_twin_stick_game_mode)
  (set `/Game/Variant_TwinStick/Blueprints/BP_TwinStickGameMode.Wave Index` (`self.CurrentWave`) _asbp_twin_stick_game_mode)
  (set `/Game/Variant_TwinStick/Blueprints/BP_TwinStickGameMode.Boss round` true _asbp_twin_stick_game_mode))

(fn `UserConstructionScript`)