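; Pushable puzzle block that slides a set distance horizontally along the impact normal when hit, kicking up limited dust puffs.
; After each move, a downward trace attaches it to what lies beneath through an interface, or resets it if nothing is there.
; Reset plays death dust, shrinks the block, returns it to its start location and grows it back.
; Four target markers, updated on construction and after moves, preview possible destinations in the editor.
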(event `self.ReceiveBeginPlay`
  ;[0 0 0 0.5] store the cubes' initial position
  (set `self.initial` (`self.K2_GetActorLocation`)))

(event `/Game/PuzzleMechanics/BPI_PuzzleMechanics.BPI_Reset`
  (bind _returnvalue (`self.K2_GetActorLocation`))
  (if (!= (`self.initial`) _returnvalue)
    (`self.StopEarly`)
    (`NiagaraFunctionLibrary.SpawnSystemAtLocation` "/Game/temporarykieranstuff/NG_DeathDust.NG_DeathDust" _returnvalue)
    (bind (_direction _shrink) (`Timeline|Shrink` :!via `PlayFromStart` :!label _label)
      (:`Update`
        (`SceneComponent.SetRelativeScale3D` (`self.Mesh`) (`KismetMathLibrary.VLerp` (1.0 1.0 1.0) (0.0 0.0 0.0) _shrink)))
      (:`Finished`
        (`/Engine/EditorBlueprintResources/StandardMacros.FlipFlop`
          (:`A`
            (`KismetSystemLibrary.Delay` 0.5)
            (`self.K2_SetActorLocation` (`self.initial`))
            (goto _label :!via `ReverseFromEnd`)))))))

(event `self.Mesh.OnComponentHit`
  (params (HitComponent :type "PrimitiveComponent Object Reference") (OtherActor :type "Actor Object Reference") (OtherComp :type "PrimitiveComponent Object Reference") (NormalImpulse :type "Vector Structure") (Hit :type "HitResult Structure (by ref)"))
  (bind (_returnvalue_x _returnvalue_y) (`KismetMathLibrary.BreakVector` (`KismetMathLibrary.Normal` Hit_ImpactNormal 1.0)))
  (bind _mesh (`self.Mesh`))
  (bind (_returnvalue_x_2 _returnvalue_y_2 _returnvalue_z) (`KismetMathLibrary.BreakVector` (`SceneComponent.K2_GetComponentLocation` _mesh)))
  (if (not (`self.IsMoving`))
    (set `self.before` (`SceneComponent.K2_GetComponentLocation` (`self.Mesh`)))
    (set `self.IsMoving` true)
    (bind (_direction _movement) (`Timeline|Move` :!via `PlayFromStart` :!label _label_2)
      (:`Update`
        (bind _returnvalue (`KismetMathLibrary.VLerp` (`self.before`) (+ (* (`KismetMathLibrary.MakeVector` _returnvalue_x _returnvalue_y) (`self.movement multiplier`)) (`self.before`)) _movement))
        (`SceneComponent.K2_SetWorldLocation` (`self.Box`) _returnvalue true false)
        (`/Engine/EditorBlueprintResources/StandardMacros.Do N` 5 :!label _label_3
          (:`Exit`
            (`NiagaraFunctionLibrary.SpawnSystemAtLocation` "/Game/PuzzleMechanics/particle/NS_Dust.NS_Dust" _returnvalue))))
      (:`Finished`
        (set `self.IsMoving` false)
        (`self.EDITOR:RecalculateTargets`)
        (`self.Particle Reset`)
        (bind (_outhit _returnvalue_2) (`KismetSystemLibrary.LineTraceSingle` :`Start` (`SceneComponent.K2_GetComponentLocation` _mesh) :`End` (`KismetMathLibrary.MakeVector` _returnvalue_x_2 _returnvalue_y_2 (- _returnvalue_z 9999.0)) :`TraceChannel` "TraceTypeQuery1" :`DrawDebugType` "Persistent"))
        (if _returnvalue_2
          (bind _in (message `/Game/PuzzleMechanics/BPI_PuzzleMechanics.BPI_ComponentToAttachTo` (`.HitActor` (`GameplayStatics.BreakHitResult` _outhit))))
          (`/Engine/EditorBlueprintResources/StandardMacros.IsValid` _in
            (:`Is Valid`
              (`SceneComponent.K2_AttachToComponent` (`self.Box`) _in "None" "KeepWorld" "KeepRelative" "KeepWorld" true)))
          (else
            (`self.BPI_Reset`)))))))

(event `Particle Reset`
  (goto _label_3 :!via `Reset`))

(event `StopEarly`
  (set `self.IsMoving` false)
  (goto _label_2 :!via `Stop`))

(fn `BPI_ComponentToAttachTo`
  (returns (In :type "PrimitiveComponent Object Reference"))
  (return null))

(fn `EDITOR:RecalculateTargets`
  (`|ExecutionSequence`
    (:`then_0`
      (`self.EDITOR:SetTargetLocation` (`self.target1`) 1.0))
    (:`then_1`
      (`self.EDITOR:SetTargetLocation` (`self.target2`) 0.0 1.0))
    (:`then_2`
      (`self.EDITOR:SetTargetLocation` (`self.target3`) -1.0))
    (:`then_3`
      (`self.EDITOR:SetTargetLocation` (`self.target4`) 0.0 -1.0))))

(fn `EDITOR:SetTargetLocation`
  (params (Target :type "PrimitiveComponent Object Reference") (X :type "Float (double-precision)") (Y :type "Float (double-precision)"))
  ;[0 0 0 0.5] EDITOR UTILITY: PREVIEW A CUBES' POSSIBLE MAX LOCATIONS
  (`SceneComponent.K2_SetWorldLocation` Target (+ (* (`KismetMathLibrary.MakeVector` X Y) (`self.movement multiplier`)) (`self.K2_GetActorLocation`)) false true)
  (`SceneComponent.K2_DetachFromComponent` Target "KeepWorld" "KeepWorld" "KeepWorld" true)
  (return))

(fn `UserConstructionScript`
  (`self.EDITOR:RecalculateTargets`))