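; BP_MovingObject is a puzzle mechanic that slides a mesh between its starting position and a FinalLocation when activated.
; It records the mesh's relative location at BeginPlay, and the Move timeline drives a lerp from there to the target.
; Activate plays the timeline forward or reverses it, with StayOpen blocking the reverse so the object remains moved.
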(event `self.ReceiveBeginPlay`
  (set `self.InitialLocation` (`SceneComponent.RelativeLocation` (`self.MeshToMove`))))

(event `self.Activate`
  (params (`On/Off` :type "ETimelineDirection Enum" :default "Forward"))
  (bind _stayopen (`self.StayOpen`))
  (switch `ETimelineDirection` `On/Off`
    (:`Forward`
      (if _stayopen
        (`/Engine/EditorBlueprintResources/StandardMacros.DoOnce` false
          (:`Completed`
            (bind (_direction _in_time) (`Timeline|Move` :!label _label)
              (:`Update`
                (`SceneComponent.K2_SetRelativeLocation` (`self.MeshToMove`) (`KismetMathLibrary.VLerp` (`self.InitialLocation`) (`self.FinalLocation`) _in_time) false false)))))
        (else
          (goto _label))))
    (:`Backward`
      (if (not _stayopen)
        (goto _label :!via `Reverse`)))))

(fn `UserConstructionScript`)