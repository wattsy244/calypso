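; BP_PowerableParent is the base Blueprint for puzzle objects, such as doors, that are powered by buttons or other actors.
; Each BPIPower call toggles the sending actor in CurrentProgress, prints debug totals, then compares the array length to ProgressRequired.
; AssessPower calls Activate with Forward once enough sources are present, otherwise Backward.
; Activate is an empty hook for children to override, and BPIActivate can also call it directly, bypassing the power check.
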(event `/Game/PuzzleMechanics/BPI_PuzzleMechanics.BPI_Power`
  (params (Actor :type "Actor Object Reference"))
  (bind _currentprogress (`self.CurrentProgress`))
  ;[0 0 0 0.5 10] When a button is activated, it'll add itself to the current power array. The length of this array will be used to determine how much power/progress has been made. If a button is already powering this object, it will remove itself, removing progress - Kieran
  (if (`KismetArrayLibrary.Array_Contains` (`self.CurrentProgress`) Actor)
    (`KismetArrayLibrary.Array_RemoveItem` _currentprogress Actor)
    (else
      (`KismetArrayLibrary.Array_AddUnique` _currentprogress Actor)))
  (`KismetSystemLibrary.PrintString` (`KismetStringLibrary.BuildString_Int` "" "Current Power:  " (`KismetArrayLibrary.Array_Length` (`self.CurrentProgress`))))
  (`KismetSystemLibrary.PrintString` (`KismetStringLibrary.BuildString_Int` "" "Needed:  " (`self.ProgressRequired`)))
  (`self.AssessPower`))

(event `AssessPower`
  ;[0 0 0 0.5 10] Event used to check if the length of the progress array is equal to how much progress is required. If it is, activate the door. Deactivate otherwise. - Kieran
  (if (>= (`KismetArrayLibrary.Array_Length` (`self.CurrentProgress`)) (`self.ProgressRequired`))
    (`self.Activate` "Forward")
    (else
      (`self.Activate` "Backward"))))

(event `Activate`
  (params (`On/Off` :type "ETimelineDirection Enum" :default "Forward"))
  ;[0 0 0 0.5 10] thanks polymorphism! <3 - Kieran
)

(event `/Game/PuzzleMechanics/BPI_PuzzleMechanics.BPI_Activate`
  (params (`In Direction` :type "ETimelineDirection Enum" :default "Forward"))
  ;[0 0 0 0.5 10] thanks polymorphism! <3 - Kieran
  (`self.Activate` `In Direction`))

(fn `UserConstructionScript`)