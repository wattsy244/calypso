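; BP_ConditionalDoor is a puzzle door that slides open when an actor tagged "caninteract" overlaps its collision.
; DoDoor plays or reverses the MoveDoor timeline, which offsets the Cube along X or Z according to CurrentDoorDirection.
; The auto-close Delay hangs off the timeline's Update rather than Finished, so its countdown to reversal begins as movement starts.
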(event `self.ReceiveBeginPlay`)

(event `self.Collision.OnComponentBeginOverlap`
  (params (OverlappedComponent :type "PrimitiveComponent Object Reference") (OtherActor :type "Actor Object Reference") (OtherComp :type "PrimitiveComponent Object Reference") (OtherBodyIndex :type Integer) (bFromSweep :type Boolean) (SweepResult :type "HitResult Structure (by ref)"))
  (if (`self.ActorHasTag` OtherActor "caninteract")
    (`self.DoDoor` "Forward")))

(event `DoDoor`
  (params (`In Direction` :type "ETimelineDirection Enum" :default "Forward"))
  ; DoorOpenClose
  (switch `ETimelineDirection` `In Direction`
    (:`Forward`
      (bind (_direction _positive) (`Timeline|MoveDoor` :!label _label)
        (:`Update`
          (switch `/Game/PuzzleMechanics/Enums_Structs/Enum_DoorDirections` (`self.CurrentDoorDirection`)
            (:`NewEnumerator0`
              (`SceneComponent.K2_SetRelativeLocation` (`self.Cube`) (`KismetMathLibrary.MakeVector` (* _positive 250.0) 0.0 80.0) false false))
            (:`NewEnumerator1`
              (`SceneComponent.K2_SetRelativeLocation` (`self.Cube`) (`KismetMathLibrary.MakeVector` (* _positive -250.0) 0.0 80.0) false false))
            (:`NewEnumerator2`
              (`SceneComponent.K2_SetRelativeLocation` (`self.Cube`) (`KismetMathLibrary.MakeVector` 0.0 0.0 (+ (* _positive 250.0) 80.0)) false false))
            (:`NewEnumerator3`
              (`SceneComponent.K2_SetRelativeLocation` (`self.Cube`) (`KismetMathLibrary.MakeVector` 0.0 0.0 (+ (* _positive -250.0) 80.0)) false false)))
          (`KismetSystemLibrary.Delay` 3.0)
          (`self.DoDoor` "Backward"))))
    (:`Backward`
      (goto _label :!via `Reverse`))))

(fn `UserConstructionScript`)